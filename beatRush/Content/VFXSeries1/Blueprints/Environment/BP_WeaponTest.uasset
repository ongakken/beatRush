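; Test weapon emitter for the VFX series that repeatedly fires configurable Kinetic, Plasma or Beam projectiles while enabled.
; BeginPlay polls Enabled, line-traces forward, pulses a glowing orb, then after a delay spawns randomly spread projectiles with optional homing on a child BP_Target.
; Tick eases that target toward the trace hit point once its simulation begins.
; The construction script uses checkbox-style flags to save or load per-type preset struct arrays in the editor.
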(event Custom|RestartOrb
  ;[1 1 1] Checks for whether the system is active and begins the automation for firing the projectile tests
  (bind _newtrack_0 (Timeline|ScaleOrb PlayFromStart)
    (:Update
      (Transformation|SetRelativeScale3D (Variables|Default|GetStaticMesh) _newtrack_0))
    (:Finished
      (CallFunction|RestartOrb)
      (Effects|SpawnEmitteratLocation "/Game/VFXSeries1/Particles/Energy/P_WeaponGlow.P_WeaponGlow" (Transformation|GetActorLocation)))))

(event Custom|CheckForEnable
  ;[1 1 1] Checks for whether the system is active and begins the automation for firing the projectile tests
  (if (Variables|ProjectileSettings|GetEnabled)
    (Utilities|FlowControl|Sequence
      (:then_0
        (Utilities|FlowControl|DoOnce false
          (:Completed
            (bind _impact_point (CallFunction|Raytrace))
            (bind _newtrack_0 (Timeline|ScaleOrb Play)
              (:Update
                (Transformation|SetRelativeScale3D (Variables|Default|GetStaticMesh) _newtrack_0))
              (:Finished
                (CallFunction|RestartOrb)
                (Effects|SpawnEmitteratLocation "/Game/VFXSeries1/Particles/Energy/P_WeaponGlow.P_WeaponGlow" (Transformation|GetActorLocation)))))))
      (:then_1
        (Utilities|FlowControl|Delay 8.0)
        (Utilities|FlowControl|DoOnce false
          (:Completed
            (CallFunction|Fireprojectile :!label _label)
            (Utilities|FlowControl|Delay (Variables|ProjectileSettings|GetDelayBetween%20Firing))
            (if (Variables|ProjectileSettings|GetEnabled)
              (CallFunction|ResetFire)
              (Variables|HiddenSettings|SetOnceStarted true)
              (else
                (CallFunction|CheckforEnable)))))))
    (else
      (Utilities|FlowControl|Delay 0.2)
      (CallFunction|CheckforEnable)
      (if (Variables|HiddenSettings|GetOnceStarted)
        (if (Variables|ProjectileSettings|GetEnabled)
          (goto _label))))))

(event Custom|ResetFire
  ;[1 1 1] Checks for whether the system is active and begins the automation for firing the projectile tests
  (CallFunction|Fireprojectile)
  (Utilities|FlowControl|Delay (Variables|ProjectileSettings|GetDelayBetween%20Firing))
  (if (Variables|ProjectileSettings|GetEnabled)
    (CallFunction|ResetFire)
    (Variables|HiddenSettings|SetOnceStarted true)
    (else
      (CallFunction|CheckforEnable))))

(event EventBeginPlay
  ;[1 1 1] Checks for whether the system is active and begins the automation for firing the projectile tests
  (if (Variables|ProjectileSettings|GetEnabled)
    (Utilities|FlowControl|Sequence
      (:then_0
        (Utilities|FlowControl|DoOnce false
          (:Completed
            (bind _impact_point (CallFunction|Raytrace))
            (bind _newtrack_0 (Timeline|ScaleOrb Play)
              (:Update
                (Transformation|SetRelativeScale3D (Variables|Default|GetStaticMesh) _newtrack_0))
              (:Finished
                (CallFunction|RestartOrb)
                (Effects|SpawnEmitteratLocation "/Game/VFXSeries1/Particles/Energy/P_WeaponGlow.P_WeaponGlow" (Transformation|GetActorLocation)))))))
      (:then_1
        (Utilities|FlowControl|Delay 8.0)
        (Utilities|FlowControl|DoOnce false
          (:Completed
            (CallFunction|Fireprojectile :!label _label)
            (Utilities|FlowControl|Delay (Variables|ProjectileSettings|GetDelayBetween%20Firing))
            (if (Variables|ProjectileSettings|GetEnabled)
              (CallFunction|ResetFire)
              (Variables|HiddenSettings|SetOnceStarted true)
              (else
                (CallFunction|CheckforEnable)))))))
    (else
      (Utilities|FlowControl|Delay 0.2)
      (CallFunction|CheckforEnable)
      (if (Variables|HiddenSettings|GetOnceStarted)
        (if (Variables|ProjectileSettings|GetEnabled)
          (goto _label))))))

(event EventTick
  (params (DeltaSeconds :type Float%20%28single-precision%29))
  (bind _bp_target (Variables|Default|GetBP_Target))
  ;[1 1 1] Checks for whether the system is active and begins the automation for firing the projectile tests
  (Variables|HiddenSettings|SetDeltatime DeltaSeconds)
  (bind _asbp_target (Utilities|Casting|CastToBP_Target (Variables|/Script/Engine.ChildActorComponent|GetChildActor (Variables|Default|GetBP_Target))))
  (if (Variables|/Game/VFXSeries1/Blueprints/Environment/BP_Target.BP_Target_C|GetBeginSimulation _asbp_target)
    (Transformation|SetWorldLocation _bp_target (Math|Interpolation|VInterpTo (Transformation|GetWorldLocation _bp_target) (stale Custom|CheckForEnable _impact_point) (Variables|HiddenSettings|GetDeltatime) 0.4) false false)))

(fn ConstructionScript
  (bind _projected_decal_size (Variables|ProjectileSettings|GetProjected%20Decal%20Size))
  ;[1 1 1] Sets the desired decal size and checks preferred projectile type to model resulting projectile behavour
  (Variables|HiddenSettings|SetDecal%20Internal (Math|Vector|MakeVector _projected_decal_size _projected_decal_size _projected_decal_size))
  (switch Utilities|FlowControl|Switch|SwitchonEnum_ProjectileType (Variables|ProjectileSettings|GetWeaponType)
    (:NewEnumerator0
      (if (Utilities|Enum|NotEqual(Enum) (Variables|ProjectileSettings|GetKineticPreset) "NewEnumerator0")
        _
        (else
          ;[1 1 1] Disables and enables the warranted projectile presets to ensure incompatiblee settings are not saved
          (Variables|ProjectileSettings|SetKineticPreset "NewEnumerator1")
          (Variables|ProjectileSettings|SetPlasmaPreset "NewEnumerator0")
          (Variables|ProjectileSettings|SetBeamPreset "NewEnumerator0")))
      ;[1 1 1] Saves the assigned settings to a struct and then unchecks appropriate check boxes once finished
      (if (Variables|ProjectileSettings|GetSave%20Pre-Load)
        (Variables|ProjectileSettings|SetSave%20Pre-Load false)
        (CallFunction|SaveKinetic)
        (elif (Variables|ProjectileSettings|GetLoad%20Pre-saved)
          (Variables|ProjectileSettings|SetLoad%20Pre-saved false)
          (CallFunction|LoadKinetic))))
    (:NewEnumerator1
      (if (Utilities|Enum|NotEqual(Enum) (Variables|ProjectileSettings|GetPlasmaPreset) "NewEnumerator0")
        _
        (else
          (Variables|ProjectileSettings|SetPlasmaPreset "NewEnumerator1")
          (Variables|ProjectileSettings|SetKineticPreset "NewEnumerator0")
          (Variables|ProjectileSettings|SetBeamPreset "NewEnumerator0")))
      (if (Variables|ProjectileSettings|GetSave%20Pre-Load)
        (Variables|ProjectileSettings|SetSave%20Pre-Load false)
        (CallFunction|SavePlasma)
        (elif (Variables|ProjectileSettings|GetLoad%20Pre-saved)
          (Variables|ProjectileSettings|SetLoad%20Pre-saved false)
          (CallFunction|LoadPlasma))))
    (:NewEnumerator2
      (if (Utilities|Enum|NotEqual(Enum) (Variables|ProjectileSettings|GetBeamPreset) "NewEnumerator0")
        _
        (else
          (Variables|ProjectileSettings|SetBeamPreset "NewEnumerator1")
          (Variables|ProjectileSettings|SetKineticPreset "NewEnumerator0")
          (Variables|ProjectileSettings|SetPlasmaPreset "NewEnumerator0")))
      (if (Variables|ProjectileSettings|GetSave%20Pre-Load)
        (Variables|ProjectileSettings|SetSave%20Pre-Load false)
        (CallFunction|SaveBeam)
        (elif (Variables|ProjectileSettings|GetLoad%20Pre-saved)
          (Variables|ProjectileSettings|SetLoad%20Pre-saved false)
          (CallFunction|LoadBeam))))))

(fn Raytrace
  (bind _returnvalue (Transformation|GetActorLocation))
  ;[1 1 1] Runs a line trace from actor location to impact point
  (bind _outhit (Collision|LineTraceForObjects _returnvalue (+ _returnvalue (* (Math|Rotator|GetRotationXVector (Transformation|GetActorRotation)) 5e+03)) (Utilities|Array|MakeArray "ObjectTypeQuery1") true (Variables|HiddenSettings|GetProjectileReference) "None"))
  (return (.ImpactPoint (Collision|BreakHitResult _outhit))))

(fn Fireprojectile
  (bind _projectilespread (Variables|ProjectileSettings|GetProjectileSpread))
  (bind _staticmesh (Variables|Default|GetStaticMesh))
  (bind _returnvalue (/ _projectilespread 2.0))
  (bind _returnvalue_2 (Transformation|GetWorldRotation _staticmesh))
  (bind (_roll _pitch _yaw) (Math|Rotator|BreakRotator _returnvalue_2))
  ;[1 1 1] Sets the spawn location to a random radius for the next fired projectile
  (Variables|HiddenSettings|SetMinSpread (* _returnvalue -1.0))
  (Variables|HiddenSettings|SetMaxSpread _returnvalue)
  ;[1 1 1] Spawns projectile and sets the resulting decal size
  (bind _returnvalue_3 (Game|SpawnActorfromClass (Variables|ProjectileSettings|GetProjectileType) (Math|Transform|MakeTransform (Transformation|GetWorldLocation _staticmesh) (Math|Rotator|MakeRotator (+ _roll (Math|Random|RandomFloatinRange (Variables|HiddenSettings|GetMinSpread) (Variables|HiddenSettings|GetMaxSpread))) (+ _pitch (Math|Random|RandomFloatinRange (Variables|HiddenSettings|GetMinSpread) (Variables|HiddenSettings|GetMaxSpread))) (+ _yaw (Math|Random|RandomFloatinRange (Variables|HiddenSettings|GetMinSpread) (Variables|HiddenSettings|GetMaxSpread))))) "Undefined" 0 "NewEnumerator0" 0))
  (Variables|/Game/VFXSeries1/Blueprints/BP_BaseProjectile.BP_BaseProjectile_C|SetDecalSize _returnvalue_3 (Variables|HiddenSettings|GetDecal%20Internal))
  (Components|StaticMesh|SetStaticMesh (Variables|/Game/VFXSeries1/Blueprints/BP_BaseProjectile.BP_BaseProjectile_C|GetProjectileMesh _returnvalue_3) (Variables|ProjectileComponents|GetSet%20Static%20Mesh))
  ;[1 1 1] Sets projectile type and ricochet preference
  (Variables|/Game/VFXSeries1/Blueprints/BP_BaseProjectile.BP_BaseProjectile_C|SetProjectileType _returnvalue_3 (Variables|ProjectileSettings|GetWeaponType))
  (Variables|/Game/VFXSeries1/Blueprints/BP_BaseProjectile.BP_BaseProjectile_C|SetRicochet _returnvalue_3 (Variables|ProjectileSettings|GetRicochet))
  ;[1 1 1] Sets the projectile particles and homing target
  (Variables|/Game/VFXSeries1/Blueprints/BP_BaseProjectile.BP_BaseProjectile_C|SetImpactParticle _returnvalue_3 (Variables|ProjectileComponents|GetImpact%20Particle))
  (Variables|/Game/VFXSeries1/Blueprints/BP_BaseProjectile.BP_BaseProjectile_C|SetHoming _returnvalue_3 (Variables|ProjectileSettings|GetTrackedProjectiles))
  (Variables|/Game/VFXSeries1/Blueprints/BP_BaseProjectile.BP_BaseProjectile_C|SetTrailParticle _returnvalue_3 (Variables|ProjectileComponents|GetProjectileTrail))
  (Variables|/Script/Engine.ProjectileMovementComponent|SetHomingTargetComponent (Variables|/Game/VFXSeries1/Blueprints/BP_BaseProjectile.BP_BaseProjectile_C|GetProjectileMovement _returnvalue_3) (Variables|Default|GetBP_Target))
  (Variables|/Script/Engine.ProjectileMovementComponent|SetHomingAccelerationMagnitude (Variables|/Game/VFXSeries1/Blueprints/BP_BaseProjectile.BP_BaseProjectile_C|GetProjectileMovement _returnvalue_3) (Variables|ProjectileSettings|GetTrackingMagnitude)))

(fn LoadKinetic
  (bind _kineticconfig (Variables|HiddenSettings|GetKineticConfig))
  (bind _kineticpreset (Variables|ProjectileSettings|GetKineticPreset))
  (bind _returnvalue (Math|Conversions|ToInteger(Byte) _kineticpreset))
  (bind _item (Utilities|Array|Get(acopy) _kineticconfig _returnvalue))
  ;[1 1 1] Calls from the User set stored Struct the saved settings for the Kinetic preset
  (Utilities|FlowControl|Sequence
    (:then_0
      (Variables|ProjectileSettings|SetProjectileName (.projectilename _item))
      (Variables|ProjectileSettings|SetWeaponType (.projectiletype _item)))
    (:then_1
      (Variables|ProjectileSettings|SetRicochet (.ricochet _item))
      (Variables|ProjectileSettings|SetTrackedProjectiles (.tracking _item)))
    (:then_2
      (Variables|ProjectileSettings|SetTrackingMagnitude (.trackingmagnitude _item))
      (Variables|ProjectileSettings|SetGravityScale (.gravityscale _item)))
    (:then_3
      (Variables|ProjectileSettings|SetProjectileSpread (.projectilespread _item))
      (Variables|ProjectileSettings|SetDelayBetween%20Firing (.rateoffire _item)))
    (:then_4
      (Variables|ProjectileSettings|SetDamage (.damage _item))
      (Variables|ProjectileComponents|SetImpactSound (.impactsound _item)))
    (:then_5
      (Variables|ProjectileComponents|SetImpact%20Particle (.impacteffect _item))
      (Variables|ProjectileComponents|SetProjectileTrail (.taileffect _item)))
    (:then_6
      (Variables|ProjectileComponents|SetSet%20Static%20Mesh (.staticmesh _item))
      (Variables|ProjectileSettings|SetProjectileScale (.projectilescale _item)))
    (:then_7
      (Variables|ProjectileSettings|SetProjectileScale (.decalsize _item))
      (Variables|ProjectileSettings|SetDecalClass (.decalclass _item)))))

(fn LoadPlasma
  (bind _plasmapreset (Variables|ProjectileSettings|GetPlasmaPreset))
  (bind _plasmaconfig (Variables|HiddenSettings|GetPlasmaConfig))
  (bind _returnvalue (Math|Conversions|ToInteger(Byte) _plasmapreset))
  (bind _item (Utilities|Array|Get(acopy) _plasmaconfig _returnvalue))
  ;[1 1 1] Calls from the User set stored Struct the saved settings for the plasma preset
  (Utilities|FlowControl|Sequence
    (:then_0
      (Variables|ProjectileSettings|SetProjectileName (.projectilename _item)))
    (:then_1
      (Variables|ProjectileSettings|SetRicochet (.ricochet _item))
      (Variables|ProjectileSettings|SetTrackedProjectiles (.tracking _item)))
    (:then_2
      (Variables|ProjectileSettings|SetTrackingMagnitude (.trackingmagnitude _item))
      (Variables|ProjectileSettings|SetGravityScale (.gravityscale _item)))
    (:then_3
      (Variables|ProjectileSettings|SetProjectileSpread (.projectilespread _item))
      (Variables|ProjectileSettings|SetDelayBetween%20Firing (.rateoffire _item)))
    (:then_4
      (Variables|ProjectileSettings|SetDamage (.damage _item))
      (Variables|ProjectileComponents|SetImpactSound (.impactsound _item)))
    (:then_5
      (Variables|ProjectileComponents|SetImpact%20Particle (.impacteffect _item))
      (Variables|ProjectileComponents|SetProjectileTrail (.taileffect _item)))
    (:then_6
      (Variables|ProjectileComponents|SetSet%20Static%20Mesh (.staticmesh _item))
      (Variables|ProjectileSettings|SetProjectileScale (.projectilescale _item)))
    (:then_7
      (Variables|ProjectileSettings|SetProjectileScale (.decalsize _item))
      (Variables|ProjectileSettings|SetDecalClass (.decalclass _item)))))

(fn LoadBeam
  (bind _beampreset (Variables|ProjectileSettings|GetBeamPreset))
  (bind _beamconfig (Variables|HiddenSettings|GetBeamConfig))
  (bind _returnvalue (Math|Conversions|ToInteger(Byte) _beampreset))
  (bind _item (Utilities|Array|Get(acopy) _beamconfig _returnvalue))
  ;[1 1 1] Calls from the User set stored Struct the saved settings for the Beam preset
  (Utilities|FlowControl|Sequence
    (:then_0
      (Variables|ProjectileSettings|SetProjectileName (.projectilename _item)))
    (:then_1
      (Variables|ProjectileSettings|SetRicochet (.ricochet _item))
      (Variables|ProjectileSettings|SetTrackedProjectiles (.tracking _item)))
    (:then_2
      (Variables|ProjectileSettings|SetTrackingMagnitude (.trackingmagnitude _item))
      (Variables|ProjectileSettings|SetGravityScale (.gravityscale _item)))
    (:then_3
      (Variables|ProjectileSettings|SetProjectileSpread (.projectilespread _item))
      (Variables|ProjectileSettings|SetDelayBetween%20Firing (.rateoffire _item)))
    (:then_4
      (Variables|ProjectileSettings|SetDamage (.damage _item))
      (Variables|ProjectileComponents|SetImpactSound (.impactsound _item)))
    (:then_5
      (Variables|ProjectileComponents|SetImpact%20Particle (.impacteffect _item))
      (Variables|ProjectileComponents|SetProjectileTrail (.taileffect _item)))
    (:then_6
      (Variables|ProjectileComponents|SetSet%20Static%20Mesh (.staticmesh _item))
      (Variables|ProjectileSettings|SetProjectileScale (.projectilescale _item)))
    (:then_7
      (Variables|ProjectileSettings|SetProjectileScale (.decalsize _item))
      (Variables|ProjectileSettings|SetDecalClass (.decalclass _item)))))

(fn SaveKinetic
  ;[1 1 1] Saves the Kinetic preferences to a struct and disables alternative behavour types
  (Utilities|Array|SetArrayElem (Variables|HiddenSettings|GetKineticConfig) (Math|Conversions|ToInteger(Byte) (Variables|ProjectileSettings|GetKineticPreset)) (Utilities|Struct|MakeStruct_KineticBaseValues (Variables|ProjectileSettings|GetProjectileName) (Variables|ProjectileSettings|GetWeaponType) (Variables|ProjectileSettings|GetRicochet) (Variables|ProjectileSettings|GetTrackedProjectiles) (Variables|ProjectileSettings|GetTrackingMagnitude) (Variables|ProjectileSettings|GetGravityScale) (Variables|ProjectileSettings|GetProjectileSpread) (Variables|ProjectileSettings|GetDelayBetween%20Firing) (Variables|ProjectileSettings|GetDamage) (Variables|ProjectileComponents|GetImpactSound) (Variables|ProjectileComponents|GetImpact%20Particle) (Variables|ProjectileComponents|GetProjectileTrail) (Variables|ProjectileComponents|GetSet%20Static%20Mesh) (Variables|ProjectileSettings|GetProjectileScale) (Variables|ProjectileSettings|GetDecalSize) (Variables|ProjectileSettings|GetDecalClass)))
  (Variables|ProjectileSettings|SetPlasmaPreset "NewEnumerator0")
  (Variables|ProjectileSettings|SetBeamPreset "NewEnumerator0"))

(fn SavePlasma
  ;[1 1 1] Saves the Plasma preferences to a struct and disables alternative behavour types
  (Utilities|Array|SetArrayElem (Variables|HiddenSettings|GetPlasmaConfig) (Math|Conversions|ToInteger(Byte) (Variables|ProjectileSettings|GetPlasmaPreset)) (Utilities|Struct|MakeStruct_PlasmaBaseValues (Variables|ProjectileSettings|GetProjectileName) (Variables|ProjectileSettings|GetWeaponType) (Variables|ProjectileSettings|GetRicochet) (Variables|ProjectileSettings|GetTrackedProjectiles) (Variables|ProjectileSettings|GetTrackingMagnitude) (Variables|ProjectileSettings|GetGravityScale) (Variables|ProjectileSettings|GetProjectileSpread) (Variables|ProjectileSettings|GetDelayBetween%20Firing) (Variables|ProjectileSettings|GetDamage) (Variables|ProjectileComponents|GetImpactSound) (Variables|ProjectileComponents|GetImpact%20Particle) (Variables|ProjectileComponents|GetProjectileTrail) (Variables|ProjectileComponents|GetSet%20Static%20Mesh) (Variables|ProjectileSettings|GetProjectileScale) (Variables|ProjectileSettings|GetDecalSize) (Variables|ProjectileSettings|GetDecalClass)))
  (Variables|ProjectileSettings|SetKineticPreset "NewEnumerator0")
  (Variables|ProjectileSettings|SetBeamPreset "NewEnumerator0"))

(fn SaveBeam
  ;[1 1 1] Saves the Beam preferences to a struct and disables alternative behavour types
  (Utilities|Array|SetArrayElem (Variables|HiddenSettings|GetBeamConfig) (Math|Conversions|ToInteger(Byte) (Variables|ProjectileSettings|GetBeamPreset)) (Utilities|Struct|MakeStruct_BeamBaseValues (Variables|ProjectileSettings|GetProjectileName) (Variables|ProjectileSettings|GetWeaponType) (Variables|ProjectileSettings|GetRicochet) (Variables|ProjectileSettings|GetTrackedProjectiles) (Variables|ProjectileSettings|GetTrackingMagnitude) (Variables|ProjectileSettings|GetGravityScale) (Variables|ProjectileSettings|GetProjectileSpread) (Variables|ProjectileSettings|GetDelayBetween%20Firing) (Variables|ProjectileSettings|GetDamage) (Variables|ProjectileComponents|GetImpactSound) (Variables|ProjectileComponents|GetImpact%20Particle) (Variables|ProjectileComponents|GetProjectileTrail) (Variables|ProjectileComponents|GetSet%20Static%20Mesh) (Variables|ProjectileSettings|GetProjectileScale) (Variables|ProjectileSettings|GetDecalSize) (Variables|ProjectileSettings|GetDecalClass)))
  (Variables|ProjectileSettings|SetKineticPreset "NewEnumerator0")
  (Variables|ProjectileSettings|SetPlasmaPreset "NewEnumerator0"))