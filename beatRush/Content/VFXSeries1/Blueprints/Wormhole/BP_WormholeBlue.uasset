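; Blue wormhole portal that pairs with a connected wormhole to show scene-capture views through its ring material.
; Construction creates the dynamic material and assigns two render targets across the pair based on Switch, which also gates the texture assignment.
; BeginPlay sets the partner capture's FOV once from player distance.
; Tick passes a smoothed, pitch-damped look-at toward the player or demo camera to the partner, and rotates its own capture by its stored rotation.
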(event EventBeginPlay
  (bind _connectedwormhole (Variables|Default|GetConnectedWormhole))
  (bind _returnvalue (Actor|GetComponentbyClass _connectedwormhole "/Script/Engine.SceneCaptureComponent2D"))
  ;[1 1 1] Checks player distance from portal and sets Field of view to scale with distance
  (Variables|Default|SetSpawnRotation (Transformation|GetActorRotation))
  (Utilities|IsValid (Variables|Default|GetP_Wormhole01)
    (:Is%20Valid
      (Utilities|IsValid _returnvalue
        (:Is%20Valid
          (Variables|/Script/Engine.SceneCaptureComponent2D|SetFOVAngle _returnvalue (- 6e+01 (/ (Transformation|GetDistanceTo (Game|Player|GetPlayerPawn 0) self) 3e+01))))))))

(event EventTick
  (params (DeltaSeconds :type Float%20%28single-precision%29))
  (bind _scenecapture2d (Variables|Default|GetSceneCapture2D))
  (bind _spawnrotation (Variables|Default|GetSpawnRotation))
  (bind _connectedwormhole (Variables|Default|GetConnectedWormhole))
  (bind (_roll _pitch _yaw) (Math|Rotator|BreakRotator _spawnrotation))
  ;[1 1 1] Checks whether the scene is in demo mode and then sets the actor the wormholes track
  (Variables|Default|SetDeltaTime DeltaSeconds)
  (if (Variables|Default|GetDemo)
    (Variables|Default|SetActorFollow (Variables|Default|GetPreviewCam))
    (else
      (Variables|Default|SetActorFollow (Game|Player|GetPlayerPawn 0))))
  ;[1 1 1] Sets entry portal camera rotation to the value obtained below
  (Utilities|IsValid _connectedwormhole
    (:Is%20Valid
      (Variables|/Game/VFXSeries1/Blueprints/Wormhole/BP_WormholeRed.BP_WormholeRed_C|SetNewRotation _connectedwormhole (Math|Rotator|MakeRotator 0.0 (- (* (.Pitch (Math|Rotator|BreakRotator (Math|Interpolation|RInterpTo (Transformation|GetWorldRotation _scenecapture2d) (Math|Rotator|FindLookatRotation (Transformation|GetWorldLocation _scenecapture2d) (Transformation|GetActorLocation (Variables|Default|GetActorFollow))) (Variables|Default|GetDeltaTime) (Variables|Default|GetRotationspeed)))) -0.25) _pitch) (- (* (.Yaw (Math|Rotator|BreakRotator (Math|Interpolation|RInterpTo (Transformation|GetWorldRotation _scenecapture2d) (Math|Rotator|FindLookatRotation (Transformation|GetWorldLocation _scenecapture2d) (Transformation|GetActorLocation (Variables|Default|GetActorFollow))) (Variables|Default|GetDeltaTime) (Variables|Default|GetRotationspeed)))) 1.0) _yaw)))
      ;[1 1 1] Checks whether the camera rotation is equal to the one stored
      (Utilities|IsValid (Variables|Default|GetSceneCapture2D)
        (:Is%20Valid
          (Transformation|SetRelativeRotation (Variables|Default|GetSceneCapture2D) (Variables|Default|GetNewRotation) false true))))))

(fn ConstructionScript
  (bind _connectedwormhole (Variables|Default|GetConnectedWormhole))
  (bind _returnvalue (Rendering|Material|CreateDynamicMaterialInstance (Variables|Default|GetP_Wormhole01) 2 "/Game/VFXSeries1/Materials/Lightning/M_PortalRingBlue.M_PortalRingBlue" :!class /Script/Engine.PrimitiveComponent))
  (Variables|Default|SetWormholeDynamicMaterial _returnvalue)
  (if (Variables|Default|GetSwitch)
    (Rendering|Material|SetTextureParameterValue (Variables|Default|GetWormholeDynamicMaterial) "Camera" "/Game/VFXSeries1/Textures/RenderCameras/RT_RenderTargetPortal01.RT_RenderTargetPortal01")
    (Rendering|Material|SetTextureParameterValue (Variables|/Game/VFXSeries1/Blueprints/Wormhole/BP_WormholeRed.BP_WormholeRed_C|GetWormholeDynamicMaterial _connectedwormhole) "Camera" "/Game/VFXSeries1/Textures/RenderCameras/RT_RenderTargetPortal02.RT_RenderTargetPortal02")
    (Variables|/Script/Engine.SceneCaptureComponent2D|SetTextureTarget (Actor|GetComponentbyClass _connectedwormhole "/Script/Engine.SceneCaptureComponent2D") "/Game/VFXSeries1/Textures/RenderCameras/RT_RenderTargetPortal02.RT_RenderTargetPortal02")
    (Variables|/Script/Engine.SceneCaptureComponent2D|SetTextureTarget (Actor|GetComponentbyClass "/Script/Engine.SceneCaptureComponent2D") "/Game/VFXSeries1/Textures/RenderCameras/RT_RenderTargetPortal01.RT_RenderTargetPortal01")
    (else
      ;[1 1 1] Sets the render target so that the connected particle will display the image captured by the scene capture in this blueprint
      (Variables|/Script/Engine.SceneCaptureComponent2D|SetTextureTarget (Actor|GetComponentbyClass _connectedwormhole "/Script/Engine.SceneCaptureComponent2D") "/Game/VFXSeries1/Textures/RenderCameras/RT_RenderTargetPortal01.RT_RenderTargetPortal01")
      (Variables|/Script/Engine.SceneCaptureComponent2D|SetTextureTarget (Actor|GetComponentbyClass "/Script/Engine.SceneCaptureComponent2D") "/Game/VFXSeries1/Textures/RenderCameras/RT_RenderTargetPortal02.RT_RenderTargetPortal02"))))