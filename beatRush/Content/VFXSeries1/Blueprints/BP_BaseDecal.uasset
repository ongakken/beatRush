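; Base VFX decal actor that spawns a randomized mark, with an optional fading energy glow.
; On BeginPlay it rotates the actor, creates a dynamic material instance, then randomizes its textures and bitmap rotation.
; Energy decals run timelines driving glow and lerp parameters, then self-destroy after a delay; others stay unlit.
; A trigger overlap calls attach on the overlapping actor with no parent specified.
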(event OnComponentBeginOverlap(TriggerVolume)
  (params (OverlappedComponent :type Primitive%20Component%20Object%20Reference) (OtherActor :type Actor%20Object%20Reference) (OtherComp :type Primitive%20Component%20Object%20Reference) (OtherBodyIndex :type Integer) (bFromSweep :type Boolean) (SweepResult :type Hit%20Result%20Structure%20%28by%20ref%29))
  ;[1 1 1] Attaches decal to actor
  (Transformation|AttachActorToActor OtherActor 0 "None" "KeepWorld" "KeepWorld" "KeepRelative" true))

(event EventBeginPlay
  (bind _decal1 (Variables|Default|GetDecal1))
  (Transformation|AddActorLocalRotation "90.000000,0.000000,90.000000" false false)
  ;[1 1 1] Set decal material and create a dynamic material instance to allow the material to have gradual fade
  (Rendering|Components|Decal|SetDecalMaterial _decal1 (Variables|Default|GetDecalMaterial))
  (bind _returnvalue (Rendering|Material|CreateDynamicMaterialInstance _decal1 :!class /Script/Engine.DecalComponent))
  (bind _output_get (Variables|Default|SetDynamicMaterialInstance _returnvalue))
  ;[1 1 1] Sets decal colour to defined
  ;  base colour
  (Rendering|Material|SetVectorParameterValue _output_get "GlowColour" (Variables|Default|GetDecalGlowBaseColour) :!class /Script/Engine.MaterialInstanceDynamic)
  ;[1 1 1] Triggers the decal randomization and also rotates
  ; bitmaps to a random rotation
  (CallFunction|RandomizeDecal)
  (Rendering|Material|SetScalarParameterValue (Variables|Default|GetDynamicMaterialInstance) "RandomRotate" (Math|Random|RandomFloatinRange 0.0 0.25) :!class /Script/Engine.MaterialInstanceDynamic)
  (if (Variables|Default|GetEnergy?)
    (Utilities|FlowControl|Sequence
      (:then_0
        ;[1 1 1] Uses timeline to alter the emissive output of the decal and
        ;  alters the lerp level to display alternative glow source
        (bind _lerptime (Timeline|DecalLerp PlayFromStart)
          (:Update
            (Rendering|Material|SetScalarParameterValue (Variables|Default|GetDynamicMaterialInstance) "Lerp" _lerptime :!class /Script/Engine.MaterialInstanceDynamic))))
      (:then_1
        (bind _burnglowtime (Timeline|DecalGlowTime PlayFromStart)
          (:Update
            (Rendering|Material|SetScalarParameterValue (Variables|Default|GetDynamicMaterialInstance) "BurnGlow" _burnglowtime :!class /Script/Engine.MaterialInstanceDynamic))
          (:Finished
            ;[1 1 1] Delays 2 seconds and destroys actor
            (Utilities|FlowControl|Delay 4.0)
            (Actor|DestroyActor)))))
    (else
      ;[1 1 1] Sets material to show no emissive glow
      (Rendering|Material|SetScalarParameterValue (Variables|Default|GetDynamicMaterialInstance) "BurnGlow" 0.0 :!class /Script/Engine.MaterialInstanceDynamic)
      (Rendering|Material|SetScalarParameterValue (Variables|Default|GetDynamicMaterialInstance) "Lerp" 1.0 :!class /Script/Engine.MaterialInstanceDynamic))))

(fn ConstructionScript)

(fn RandomizeDecal
  (bind _basecolour (Variables|Default|GetBaseColour))
  (bind _emissive (Variables|Default|Getemissive))
  (bind _normals (Variables|Default|GetNormals))
  ;[1 1 1] Randomly selects new bitmaps from array and dynamically changes decal output on spawn
  (Rendering|Material|SetTextureParameterValue (Variables|Default|GetDynamicMaterialInstance) "DecalTexture" (Utilities|Array|Get(acopy) _basecolour (Math|Random|RandomIntegerinRange 0 (Utilities|Array|Length _basecolour))))
  (Rendering|Material|SetTextureParameterValue (Variables|Default|GetDynamicMaterialInstance) "GlowUnderLay" (Utilities|Array|Get(acopy) _emissive (Math|Random|RandomIntegerinRange 0 (Utilities|Array|Length _emissive))))
  (Rendering|Material|SetTextureParameterValue (Variables|Default|GetDynamicMaterialInstance) "Normal" (Utilities|Array|Get(acopy) _normals (Math|Random|RandomIntegerinRange 0 (Utilities|Array|Length _normals))))
  (return))