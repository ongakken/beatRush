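; BP_SB4K_HD_Echvora is a placeable space skybox actor showing the HD Echvora backdrop from the SpaceBox Color set.
; Its construction script sets the actor's scale from a Scale variable and assigns a dedicated Echvora material to each of the six face components: Up, Down, Left, Right, Front and Back.
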(fn ConstructionScript
  (Transformation|SetActorScale3D (Variables|Default|GetScale))
  (Rendering|Material|SetMaterial (Variables|Default|GetUp) 0 "/Game/SpaceBox_Color/Materials/HD/Echvora/Mat_HD_Echvora_Up.Mat_HD_Echvora_Up")
  (Rendering|Material|SetMaterial (Variables|Default|GetRight) 0 "/Game/SpaceBox_Color/Materials/HD/Echvora/Mat_HD_Echvora_Right.Mat_HD_Echvora_Right")
  (Rendering|Material|SetMaterial (Variables|Default|GetLeft) 0 "/Game/SpaceBox_Color/Materials/HD/Echvora/Mat_HD_Echvora_Left.Mat_HD_Echvora_Left")
  (Rendering|Material|SetMaterial (Variables|Default|GetFront) 0 "/Game/SpaceBox_Color/Materials/HD/Echvora/Mat_HD_Echvora_Front.Mat_HD_Echvora_Front")
  (Rendering|Material|SetMaterial (Variables|Default|GetDown) 0 "/Game/SpaceBox_Color/Materials/HD/Echvora/Mat_HD_Echvora_Down.Mat_HD_Echvora_Down")
  (Rendering|Material|SetMaterial (Variables|Default|GetBack) 0 "/Game/SpaceBox_Color/Materials/HD/Echvora/Mat_HD_Echvora_Back.Mat_HD_Echvora_Back"))