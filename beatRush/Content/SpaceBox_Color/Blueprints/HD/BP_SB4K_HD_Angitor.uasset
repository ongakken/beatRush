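; BP_SB4K_HD_Angitor is a space skybox actor from the SpaceBox_Color set, showing the HD Angitor variant.
; Its construction script sets the actor's scale from the Scale variable.
; It then assigns a dedicated Angitor material to each of the six face components: Up, Down, Left, Right, Front and Back.
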(fn ConstructionScript
  (Transformation|SetActorScale3D (Variables|Default|GetScale))
  (Rendering|Material|SetMaterial (Variables|Default|GetUp) 0 "/Game/SpaceBox_Color/Materials/HD/Angitor/Mat_HD_Angitor_Up.Mat_HD_Angitor_Up")
  (Rendering|Material|SetMaterial (Variables|Default|GetRight) 0 "/Game/SpaceBox_Color/Materials/HD/Angitor/Mat_HD_Angitor_Right.Mat_HD_Angitor_Right")
  (Rendering|Material|SetMaterial (Variables|Default|GetLeft) 0 "/Game/SpaceBox_Color/Materials/HD/Angitor/Mat_HD_Angitor_Left.Mat_HD_Angitor_Left")
  (Rendering|Material|SetMaterial (Variables|Default|GetFront) 0 "/Game/SpaceBox_Color/Materials/HD/Angitor/Mat_HD_Angitor_Front.Mat_HD_Angitor_Front")
  (Rendering|Material|SetMaterial (Variables|Default|GetDown) 0 "/Game/SpaceBox_Color/Materials/HD/Angitor/Mat_HD_Angitor_Down.Mat_HD_Angitor_Down")
  (Rendering|Material|SetMaterial (Variables|Default|GetBack) 0 "/Game/SpaceBox_Color/Materials/HD/Angitor/Mat_HD_Angitor_Back.Mat_HD_Angitor_Back"))