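; BP_SB4K_HD_Ryrak is a space skybox actor from the SpaceBox_Color set, showing the HD Ryrak backdrop on six cube faces.
; Its construction script scales the actor by the Scale variable, then assigns a dedicated Ryrak material to each Up, Down, Left, Right, Front and Back component.
; All setup happens in the construction script, with no runtime logic.
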(fn ConstructionScript
  (Transformation|SetActorScale3D (Variables|Default|GetScale))
  (Rendering|Material|SetMaterial (Variables|Default|GetUp) 0 "/Game/SpaceBox_Color/Materials/HD/Ryrak/Mat_HD_Ryrak_Up.Mat_HD_Ryrak_Up")
  (Rendering|Material|SetMaterial (Variables|Default|GetRight) 0 "/Game/SpaceBox_Color/Materials/HD/Ryrak/Mat_HD_Ryrak_Right.Mat_HD_Ryrak_Right")
  (Rendering|Material|SetMaterial (Variables|Default|GetLeft) 0 "/Game/SpaceBox_Color/Materials/HD/Ryrak/Mat_HD_Ryrak_Left.Mat_HD_Ryrak_Left")
  (Rendering|Material|SetMaterial (Variables|Default|GetFront) 0 "/Game/SpaceBox_Color/Materials/HD/Ryrak/Mat_HD_Ryrak_Front.Mat_HD_Ryrak_Front")
  (Rendering|Material|SetMaterial (Variables|Default|GetDown) 0 "/Game/SpaceBox_Color/Materials/HD/Ryrak/Mat_HD_Ryrak_Down.Mat_HD_Ryrak_Down")
  (Rendering|Material|SetMaterial (Variables|Default|GetBack) 0 "/Game/SpaceBox_Color/Materials/HD/Ryrak/Mat_HD_Ryrak_Back.Mat_HD_Ryrak_Back"))