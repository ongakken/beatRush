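; BP_SB4K_HD_Lerendo is a space box actor that displays the HD Lerendo environment on six sides.
; Its construction script scales the whole actor by the Scale variable, then assigns a dedicated Lerendo material to each of the Up, Down, Left, Right, Front and Back components.
; The file shows no other logic, as all setup happens at construction.
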(fn ConstructionScript
  (Transformation|SetActorScale3D (Variables|Default|GetScale))
  (Rendering|Material|SetMaterial (Variables|Default|GetUp) 0 "/Game/SpaceBox_Color/Materials/HD/Lerendo/Mat_HD_Lerendo_Up.Mat_HD_Lerendo_Up")
  (Rendering|Material|SetMaterial (Variables|Default|GetRight) 0 "/Game/SpaceBox_Color/Materials/HD/Lerendo/Mat_HD_Lerendo_Right.Mat_HD_Lerendo_Right")
  (Rendering|Material|SetMaterial (Variables|Default|GetLeft) 0 "/Game/SpaceBox_Color/Materials/HD/Lerendo/Mat_HD_Lerendo_Left.Mat_HD_Lerendo_Left")
  (Rendering|Material|SetMaterial (Variables|Default|GetFront) 0 "/Game/SpaceBox_Color/Materials/HD/Lerendo/Mat_HD_Lerendo_Front.Mat_HD_Lerendo_Front")
  (Rendering|Material|SetMaterial (Variables|Default|GetDown) 0 "/Game/SpaceBox_Color/Materials/HD/Lerendo/Mat_HD_Lerendo_Down.Mat_HD_Lerendo_Down")
  (Rendering|Material|SetMaterial (Variables|Default|GetBack) 0 "/Game/SpaceBox_Color/Materials/HD/Lerendo/Mat_HD_Lerendo_Back.Mat_HD_Lerendo_Back"))