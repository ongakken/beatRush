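; Space skybox actor for the HD Mortino variant in the SpaceBox Color set, built from six face components.
; Its construction script scales the whole actor by a Scale variable and assigns each face (Up, Down, Left, Right, Front, Back) its matching Mortino material.
; The graph shown holds only this construction-time setup, with no runtime logic.
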(fn ConstructionScript
  (Transformation|SetActorScale3D (Variables|Default|GetScale))
  (Rendering|Material|SetMaterial (Variables|Default|GetUp) 0 "/Game/SpaceBox_Color/Materials/HD/Mortino/Mat_HD_Mortino_Up.Mat_HD_Mortino_Up")
  (Rendering|Material|SetMaterial (Variables|Default|GetRight) 0 "/Game/SpaceBox_Color/Materials/HD/Mortino/Mat_HD_Mortino_Right.Mat_HD_Mortino_Right")
  (Rendering|Material|SetMaterial (Variables|Default|GetLeft) 0 "/Game/SpaceBox_Color/Materials/HD/Mortino/Mat_HD_Mortino_Left.Mat_HD_Mortino_Left")
  (Rendering|Material|SetMaterial (Variables|Default|GetFront) 0 "/Game/SpaceBox_Color/Materials/HD/Mortino/Mat_HD_Mortino_Front.Mat_HD_Mortino_Front")
  (Rendering|Material|SetMaterial (Variables|Default|GetDown) 0 "/Game/SpaceBox_Color/Materials/HD/Mortino/Mat_HD_Mortino_Down.Mat_HD_Mortino_Down")
  (Rendering|Material|SetMaterial (Variables|Default|GetBack) 0 "/Game/SpaceBox_Color/Materials/HD/Mortino/Mat_HD_Mortino_Back.Mat_HD_Mortino_Back"))