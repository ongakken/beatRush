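; Space skybox actor for the HD Arothe variant of the SpaceBox_Color set, built from six face components: Up, Down, Left, Right, Front and Back.
; The construction script scales the whole actor by its Scale variable and assigns each face its matching Arothe material.
; The graph holds only this construction-time setup, with no runtime logic.
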(fn ConstructionScript
  (Transformation|SetActorScale3D (Variables|Default|GetScale))
  (Rendering|Material|SetMaterial (Variables|Default|GetUp) 0 "/Game/SpaceBox_Color/Materials/HD/Arothe/Mat_HD_Arothe_Up.Mat_HD_Arothe_Up")
  (Rendering|Material|SetMaterial (Variables|Default|GetRight) 0 "/Game/SpaceBox_Color/Materials/HD/Arothe/Mat_HD_Arothe_Right.Mat_HD_Arothe_Right")
  (Rendering|Material|SetMaterial (Variables|Default|GetLeft) 0 "/Game/SpaceBox_Color/Materials/HD/Arothe/Mat_HD_Arothe_Left.Mat_HD_Arothe_Left")
  (Rendering|Material|SetMaterial (Variables|Default|GetFront) 0 "/Game/SpaceBox_Color/Materials/HD/Arothe/Mat_HD_Arothe_Front.Mat_HD_Arothe_Front")
  (Rendering|Material|SetMaterial (Variables|Default|GetDown) 0 "/Game/SpaceBox_Color/Materials/HD/Arothe/Mat_HD_Arothe_Down.Mat_HD_Arothe_Down")
  (Rendering|Material|SetMaterial (Variables|Default|GetBack) 0 "/Game/SpaceBox_Color/Materials/HD/Arothe/Mat_HD_Arothe_Back.Mat_HD_Arothe_Back"))