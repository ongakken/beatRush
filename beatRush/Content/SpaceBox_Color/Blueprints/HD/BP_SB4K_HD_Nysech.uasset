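; BP_SB4K_HD_Nysech is a space skybox actor from the SpaceBox Color pack, showing the HD Nysech sky on six cube faces.
; Its construction script sets the actor's scale from the Scale variable.
; It then assigns a dedicated Nysech material to each of the Up, Down, Left, Right, Front and Back components.
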(fn ConstructionScript
  (Transformation|SetActorScale3D (Variables|Default|GetScale))
  (Rendering|Material|SetMaterial (Variables|Default|GetUp) 0 "/Game/SpaceBox_Color/Materials/HD/Nysech/Mat_HD_Nysech_Up.Mat_HD_Nysech_Up")
  (Rendering|Material|SetMaterial (Variables|Default|GetRight) 0 "/Game/SpaceBox_Color/Materials/HD/Nysech/Mat_HD_Nysech_Right.Mat_HD_Nysech_Right")
  (Rendering|Material|SetMaterial (Variables|Default|GetLeft) 0 "/Game/SpaceBox_Color/Materials/HD/Nysech/Mat_HD_Nysech_Left.Mat_HD_Nysech_Left")
  (Rendering|Material|SetMaterial (Variables|Default|GetFront) 0 "/Game/SpaceBox_Color/Materials/HD/Nysech/Mat_HD_Nysech_Front.Mat_HD_Nysech_Front")
  (Rendering|Material|SetMaterial (Variables|Default|GetDown) 0 "/Game/SpaceBox_Color/Materials/HD/Nysech/Mat_HD_Nysech_Down.Mat_HD_Nysech_Down")
  (Rendering|Material|SetMaterial (Variables|Default|GetBack) 0 "/Game/SpaceBox_Color/Materials/HD/Nysech/Mat_HD_Nysech_Back.Mat_HD_Nysech_Back"))