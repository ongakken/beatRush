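; Player controller for the point cloud morphing demo that lets number keys switch between point clouds.
; On BeginPlay it looks for a BP_DemoControls actor, caching it and flagging the level as the control demo map if found.
; On that map, keys 1 to 6 each pass a zero-based cloud index to the actor's PlayMorphFromTo; elsewhere they do nothing.
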(event EventBeginPlay
  ;[1 1 1] Search BP_DemoControl actor on the level. If successful then mean that is Control Demo Map example
  (bind _outactors (Actor|GetAllActorsOfClass "/Game/PointCloudsMorphing/Blueprints/BP_DemoControls.BP_DemoControls_C"))
  (Utilities|IsValid (Utilities|Array|Get(acopy) _outactors)
    (:Is%20Valid
      (Variables|Default|SetIsDemoConrolMap true)
      (Variables|Default|SetDemoControlBP (Utilities|Array|Get(acopy) _outactors)))))

(event EventTick
  (params (DeltaSeconds :type Float%20%28single-precision%29)))

(event Input|KeyboardEvents|1
  (params (Key :type Key%20Structure :default "AnyKey"))
  ;[1 1 1] If this DemoControl level then switch point clouds by key press. Pass clouds indexes (from and to) to PoinCloudsControl actor
  (:Pressed
    (if (Variables|Default|GetIsDemoConrolMap)
      (Default|PlayMorphfromto (Variables|Default|GetDemoControlBP)))))

(event Input|KeyboardEvents|2
  (params (Key :type Key%20Structure :default "AnyKey"))
  ;[1 1 1] If this DemoControl level then switch point clouds by key press. Pass clouds indexes (from and to) to PoinCloudsControl actor
  (:Pressed
    (if (Variables|Default|GetIsDemoConrolMap)
      (Default|PlayMorphfromto (Variables|Default|GetDemoControlBP) 1))))

(event Input|KeyboardEvents|3
  (params (Key :type Key%20Structure :default "AnyKey"))
  ;[1 1 1] If this DemoControl level then switch point clouds by key press. Pass clouds indexes (from and to) to PoinCloudsControl actor
  (:Pressed
    (if (Variables|Default|GetIsDemoConrolMap)
      (Default|PlayMorphfromto (Variables|Default|GetDemoControlBP) 2))))

(event Input|KeyboardEvents|4
  (params (Key :type Key%20Structure :default "AnyKey"))
  ;[1 1 1] If this DemoControl level then switch point clouds by key press. Pass clouds indexes (from and to) to PoinCloudsControl actor
  (:Pressed
    (if (Variables|Default|GetIsDemoConrolMap)
      (Default|PlayMorphfromto (Variables|Default|GetDemoControlBP) 3))))

(event Input|KeyboardEvents|5
  (params (Key :type Key%20Structure :default "AnyKey"))
  ;[1 1 1] If this DemoControl level then switch point clouds by key press. Pass clouds indexes (from and to) to PoinCloudsControl actor
  (:Pressed
    (if (Variables|Default|GetIsDemoConrolMap)
      (Default|PlayMorphfromto (Variables|Default|GetDemoControlBP) 4))))

(event Input|KeyboardEvents|6
  (params (Key :type Key%20Structure :default "AnyKey"))
  ;[1 1 1] If this DemoControl level then switch point clouds by key press. Pass clouds indexes (from and to) to PoinCloudsControl actor
  (:Pressed
    (if (Variables|Default|GetIsDemoConrolMap)
      (Default|PlayMorphfromto (Variables|Default|GetDemoControlBP) 5))))

(fn ConstructionScript)