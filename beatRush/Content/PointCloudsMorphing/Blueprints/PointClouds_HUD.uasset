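; PointClouds_HUD is the HUD for the point cloud morphing demo, drawing an on-screen hint about switching figures with keys 1 to 6.
; On each DrawHUD it casts the player controller to PointClouds_PlayerController and draws only when that controller's IsDemoConrolMap flag is set.
; Text position and scale are derived from the screen size relative to a 1280x720 reference.
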(event EventBeginPlay)

(event Collision|EventActorBeginOverlap
  (params (OtherActor :type Actor%20Object%20Reference)))

(event EventTick
  (params (DeltaSeconds :type Float%20%28single-precision%29)))

(event EventDrawHUD
  (params (SizeX :type Integer) (SizeY :type Integer))
  ;[1 1 1] Draw text message on screen: Press 1-6 for switch figures
  (bind _aspoint_clouds_player_controller (Utilities|Casting|CastToPointClouds_PlayerController (Game|GetPlayerController 0)))
  (if (Variables|/Game/PointCloudsMorphing/Blueprints/PointClouds_PlayerController.PointClouds_PlayerController_C|GetIsDemoConrolMap _aspoint_clouds_player_controller)
    (Utilities|FlowControl|Sequence
      (:then_0
        (Variables|Default|SetHUDXRatio (/ (Math|Conversions|ToFloat(Integer) SizeX) 1.28e+03)))
      (:then_1
        (Variables|Default|SetHUDYRatio (/ (Math|Conversions|ToFloat(Integer) SizeY) 7.2e+02)))
      (:then_2
        (HUD|DrawText "Press keys 1...6 for switch figure" "(R=0.933698,G=0.985000,B=0.985000,A=1.000000)" (* 1e+01 (Variables|Default|GetHUDXRatio)) (* 2e+01 (Variables|Default|GetHUDYRatio)) "/Engine/EngineFonts/Roboto.Roboto" (* 1.5 (Variables|Default|GetHUDYRatio)) false)))))

(fn ConstructionScript)