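; Demo controller that drives a PointCloudsMorphing effect, animating its transform and switching between point clouds.
; Each tick it sends a new transform through SetMorphTransform, bobbing the effect vertically on a sine wave around its initial location while steadily yawing it.
; PlayMorphFromTo morphs from the last cloud index to a requested one, ignoring repeats and printing a notice if a morph is already running.
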(event Custom|PlayMorphFromTo
  (params (to_index :type Integer))
  (bind _pointcloudsmorphing (Variables|Default|GetPointCloudsMorphing))
  ;[1 1 1] Play morphing effect between two point clouds. Index - current index of clouds texture for play. Check if that effect currently is not in morphing state
  (if (!= (Variables|Default|GetPreviousCloudIndex) to_index)
    (if (Utilities|Enum|NotEqual(Enum) (Variables|/Game/PointCloudsMorphing/Blueprints/BP_PointCloudsMorphing.BP_PointCloudsMorphing_C|Getstate _pointcloudsmorphing) "NewEnumerator1")
      (Default|Playfromto _pointcloudsmorphing (Variables|Default|GetPreviousCloudIndex) to_index)
      (Variables|Default|SetPreviousCloudIndex to_index)
      (else
        (Development|PrintString "Morphing in progress" true true "(R=1.000000,G=0.860000,B=0.000000,A=1.000000)" 1.0)))))

(event EventBeginPlay
  ;[1 1 1] Setup initial parameters for effect controlling - location, rotation, rotation counter, start cloud texture index
  (Variables|Default|SetInit_Location (Transformation|GetActorLocation (Variables|Default|GetPointCloudsMorphing)))
  (Variables|Default|SetRotationCounter 0.0)
  (Variables|Default|SetEffectRotation 0.0)
  (Variables|Default|SetPreviousCloudIndex 0))

(event EventTick
  (params (DeltaSeconds :type Float%20%28single-precision%29))
  ;[1 1 1] Update transformation. Pass location, rotation, scale to Point Clouds Mophing
  (Variables|Default|SetRotationCounter (+ (Variables|Default|GetRotationCounter) 0.05))
  (Variables|Default|SetEffectRotation (+ (Variables|Default|GetEffectRotation) 0.15))
  ;[1 1 1] We need to call this event for change effect location, rotation and scale
  (Default|SetMorphTransform (Variables|Default|GetPointCloudsMorphing) (Math|Transform|MakeTransform (+ (Variables|Default|GetInit_Location) (Math|Vector|MakeVector 0.0 0.0 (* (Math|Trig|Sin(Radians) (Variables|Default|GetRotationCounter)) 8e+01))) (Math|Rotator|MakeRotator 0.0 0.0 (Variables|Default|GetEffectRotation)))))

(fn ConstructionScript)