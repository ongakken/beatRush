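; Player ship for Beat Rush, an auto-forward dodging game that also runs menus, level flow and saving.
; StartGame loops random spawns of health-restoring points and obstacles, with speed, spawn rate and obstacle variety scaling by LevelNum.
; Each level plays a music track; surviving a matching hard-coded Delay shows an interstitial, then saves the next level.
; BeginPlay loads progress and spawns mountain scenery; other events handle ship swaps, pickups, damage and death.
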(event Custom|getPoint
  (params (pointType :type String))
  (bind _pointsnum (Variables|Default|GetpointsNum))
  (if (Utilities|Enum|Equal(Enum) pointType "regular")
    (Math|Integer|IncrementInt _pointsnum
      (:%20%20
        (Math|Integer|IncrementInt (Variables|Default|GetregularPointsNum)
          (:%20%20
            (Audio|PlaySound2D "/Game/audio/SFX/sfx2/sfx2/access.access" 1.0 1.0 0.0 0 0)
            (Variables|Default|Sethealth (+ (Variables|Default|Gethealth) 5.0))))))
    (elif (Utilities|Enum|Equal(Enum) pointType "better")
      (Math|Integer|IncrementInt _pointsnum
        (:%20%20
          (Math|Integer|IncrementInt (Variables|Default|GetbetterPointsNum)
            (:%20%20
              (Audio|PlaySound2D "/Game/audio/SFX/sfx2/sfx2/access2.access2" 1.0 1.0 0.0 0 0)
              (Variables|Default|Sethealth (+ (Variables|Default|Gethealth) 1e+01))))))
      (elif (Utilities|Enum|Equal(Enum) pointType "simtoon")
        (Math|Integer|IncrementInt _pointsnum
          (:%20%20
            (Math|Integer|IncrementInt (Variables|Default|GetsimtoonPointsNum)
              (:%20%20
                (Audio|PlaySound2D "/Game/audio/SFX/sfx2/sfx2/access3.access3" 1.0 1.0 0.0 0 0)
                (Variables|Default|Sethealth (+ (Variables|Default|Gethealth) 15.0))))))))))

(event Custom|startGame
  (params (level :type Float%20%28single-precision%29))
  (bind _returnvalue (Math|Random|RandomFloatinRange -1e+03 1e+03))
  (bind _returnvalue_2 (Math|Random|RandomFloatinRange 1e+02 4e+02))
  (bind _returnvalue_3 (Math|Random|RandomFloatinRange -4e+02 -1e+02))
  (bind _returnvalue_4 (Math|Random|RandomIntegerinRange 0 1))
  (bind _music (Variables|Default|Getmusic))
  (bind _music_2 (Variables|Default|Getmusic))
  (bind _music_3 (Variables|Default|Getmusic))
  (bind _music_4 (Variables|Default|Getmusic))
  (bind _music_5 (Variables|Default|Getmusic))
  (bind _music_6 (Variables|Default|Getmusic))
  (bind _betterpointsarr (Variables|Default|GetbetterPointsArr))
  (bind _regularpointsarr (Variables|Default|GetregularPointsArr))
  (bind _simtoonpointsarr (Variables|Default|GetsimtoonPointsArr))
  (bind _capsulecomponent (Variables|Collision|GetCapsuleComponent))
  (bind _music_7 (Variables|Default|Getmusic))
  (bind _returnvalue_5 (Transformation|GetWorldLocation _capsulecomponent))
  (bind _relativelocation (Variables|/Script/Engine.SceneComponent|GetRelativeLocation _capsulecomponent))
  (bind _returnvalue_6 (+ (.x _returnvalue_5) -1e+04))
  (bind _returnvalue_7 (+ (.y _relativelocation) _returnvalue_2))
  (bind _returnvalue_8 (+ (.y _relativelocation) _returnvalue_3))
  (bind _returnvalue_9 (Math|Transform|MakeTransform (Math|Vector|MakeVector _returnvalue_6 _returnvalue_7 4.4e+02)))
  (bind _returnvalue_10 (Math|Transform|MakeTransform (Math|Vector|MakeVector _returnvalue_6 _returnvalue_8 4.4e+02)))
  (bind _returnvalue_11 (+ _returnvalue_8 _returnvalue))
  (Widget|RemovefromParent (Variables|Default|GetmainMenu))
  (Variables|Default|SetisGameFocused true)
  (CallFunction|RespawnPlayer)
  (Utilities|FlowControl|Sequence
    (:then_0
      (switch int (Math|Random|RandomIntegerinRange 0 2) :!label _label
        (:0
          (switch int _returnvalue_4
            (:0
              (bind _returnvalue_12 (Game|SpawnActorfromClass "/Game/BP/pointRegular_BP.pointRegular_BP_C" _returnvalue_10 "AlwaysSpawn" 0 0))
              (Utilities|Array|Add _regularpointsarr _returnvalue_12))
            (:1
              (bind _returnvalue_13 (Game|SpawnActorfromClass "/Game/BP/pointRegular_BP.pointRegular_BP_C" _returnvalue_9 "AlwaysSpawn" 0 0))
              (Utilities|Array|Add _regularpointsarr _returnvalue_13))))
        (:1
          (switch int _returnvalue_4
            (:0
              (bind _returnvalue_14 (Game|SpawnActorfromClass "/Game/BP/pointBetter_BP.pointBetter_BP_C" _returnvalue_10 "AlwaysSpawn" 0 0))
              (Utilities|Array|Add _betterpointsarr _returnvalue_14))
            (:1
              (bind _returnvalue_15 (Game|SpawnActorfromClass "/Game/BP/pointBetter_BP.pointBetter_BP_C" _returnvalue_9 "AlwaysSpawn" 0 0))
              (Utilities|Array|Add _betterpointsarr _returnvalue_15))))
        (:2
          (switch int _returnvalue_4
            (:0
              (bind _returnvalue_16 (Game|SpawnActorfromClass "/Game/BP/pointSimtoon_BP.pointSimtoon_BP_C" _returnvalue_10 "AlwaysSpawn" 0 0))
              (Utilities|Array|Add _simtoonpointsarr _returnvalue_16))
            (:1
              (bind _returnvalue_17 (Game|SpawnActorfromClass "/Game/BP/pointSimtoon_BP.pointSimtoon_BP_C" _returnvalue_9 "AlwaysSpawn" 0 0))
              (Utilities|Array|Add _simtoonpointsarr _returnvalue_17)
              (Utilities|FlowControl|Delay (/ (Math|Random|RandomFloatinRange 1.0 3.0) (Variables|Default|GetlevelNum)))
              (goto _label)))))
      (Utilities|FlowControl|Sequence
        (:then_0
          (Utilities|FlowControl|Delay (/ (Math|Random|RandomFloatinRange 1.0 3.0) (Variables|Default|GetlevelNum)))
          (switch int (Math|Random|RandomIntegerinRange 0 2) :!label _label_2
            (:0
              (bind _returnvalue_18 (Game|SpawnActorfromClass "/Game/BP/BP_obstacleVar1.BP_obstacleVar1_C" (Math|Transform|MakeTransform (Math|Vector|MakeVector (* (+ _returnvalue_6 (Math|Random|RandomFloatinRange (/ 1e+03 (Variables|Default|GetlevelNum)) 2.5e+03)) 1.1) _returnvalue_11 2.5e+02) "0, 0, 0" "2.000000,2.000000,2.000000") "AlwaysSpawn" 0 0 :!label _label_3))
              (Utilities|Array|Add (Variables|Default|GetobstacleV1Arr) _returnvalue_18)
              (Utilities|FlowControl|Delay (/ (Math|Random|RandomFloatinRange 1.0 3.0) (Variables|Default|GetlevelNum)) :!label _label_4)
              (goto _label))
            (:1
              (if (> (Variables|Default|GetlevelNum) 2.0)
                (bind _returnvalue_19 (Game|SpawnActorfromClass "/Game/BP/BP_obstacleVar2.BP_obstacleVar2_C" (Math|Transform|MakeTransform (Math|Vector|MakeVector (* (+ _returnvalue_6 (Math|Random|RandomFloatinRange (/ 1e+03 (Variables|Default|GetlevelNum)) 2.5e+03)) 1.1) _returnvalue_11 2.5e+02) "0, 0, 0" "2.000000,2.000000,2.000000") "AlwaysSpawn" 0 0))
                (Utilities|Array|Add (Variables|Default|GetobstacleV2Arr) _returnvalue_19)
                (Utilities|FlowControl|Delay (/ (Math|Random|RandomFloatinRange 1.0 3.0) (Variables|Default|GetlevelNum)))
                (goto _label_3)
                (else
                  (goto _label_3))))
            (:2
              (if (> (Variables|Default|GetlevelNum) 4.0)
                (bind _returnvalue_20 (Game|SpawnActorfromClass "/Game/BP/BP_obstacleVar3.BP_obstacleVar3_C" (Math|Transform|MakeTransform (Math|Vector|MakeVector (* (* (+ _returnvalue_6 (Math|Random|RandomFloatinRange (/ 1e+03 (Variables|Default|GetlevelNum)) 2.5e+03)) 1.1) 1.75) _returnvalue_11 2.5e+02) "0,-90.000000, 0" "2.000000,2.000000,2.000000") "AlwaysSpawn" 0 0))
                (Utilities|Array|Add (Variables|Default|GetobstacleV3Arr) _returnvalue_20)
                (else
                  (goto _label_2))))))
        (:then_1
          (goto _label_4))))
    (:then_1
      (bind _returnvalue_21 (UserInterface|CreateWidget "/Game/UI/HUD.HUD_C"))
      (bind _output_get (Variables|Default|SetHUD _returnvalue_21))
      (UserInterface|Viewport|AddtoViewport _output_get 0))
    (:then_2
      ;[0 0.957 1 1 85] Level 1
      (if (or (== (Variables|Default|GetlevelNum) 1.0) (Variables|Default|GetisReplaying)) :!label _label_5
        (Audio|Components|Audio|SetSound _music_2 "/Game/audio/OST/caffeine.caffeine")
        (Utilities|FlowControl|Sequence
          (:then_0
            (Audio|Components|Audio|Play _music_2 0.0)
            (Utilities|FlowControl|Delay 1.5e+02)
            (Audio|PlaySound2D "/Game/audio/SFX/sfx2/sfx2/accomplished2.accomplished2" 1.0 1.0 0.0 0 0)
            (Utilities|FlowControl|Delay 1.0)
            (|ShowInterstitial
              (:then
                (if (== (Variables|Default|GetlevelNum) 1.0)
                  (bind _output_get_2 (Variables|Default|SetlevelNum 2.0))
                  (bind _success_ (CallFunction|SaveALL (Variables|Default|GetsimtoonPointsNum) _output_get_2 (Variables|Default|GetcurrentShip) (Variables|Default|Getads_removed)))
                  (if _success_
                    (Audio|PlaySound2D "/Game/audio/SFX/sfx2/sfx2/accomplished3.accomplished3" 1.0 1.0 0.0 0 0)
                    (Utilities|FlowControl|Delay 0.2)
                    (Variables|Default|SetmoveUpMultiplier 1.0)
                    (Transformation|SetActorLocationAndRotation "154.399994,36.360001,3547.199951" "0, 0,-179.800003" false true)
                    (goto _label_5))))))
          (:then_1
            (Utilities|FlowControl|Delay 3.0)
            (Variables|Default|SettutorialText "Welcome!")
            (Utilities|FlowControl|Delay 2.0)
            (Variables|Default|SettutorialText "Let's keep this simple ...")
            (Utilities|FlowControl|Delay 3.0)
            (Variables|Default|SettutorialText "Those colorful shining objects are what we call 'points' ...")
            (Utilities|FlowControl|Delay 5.0)
            (Variables|Default|SettutorialText "The blue ones serve as a digital currency within the game and restore your health")
            (Utilities|FlowControl|Delay 6.0)
            (Variables|Default|SettutorialText "You can buy stuff in the Shop with them ...")
            (Utilities|FlowControl|Delay 4.0)
            (Variables|Default|SettutorialText "The other ones only restore your health")
            (Utilities|FlowControl|Delay 4.0)
            (Variables|Default|SettutorialText "The rocks you see generating ahead are obstacles ...")
            (Utilities|FlowControl|Delay 4.0)
            (Variables|Default|SettutorialText "Avoid them to survive ...")
            (Utilities|FlowControl|Delay 3.5)
            (Variables|Default|SettutorialText "Later in the game, more obstacles will begin to appear ...")
            (Utilities|FlowControl|Delay 5.0)
            (Variables|Default|SettutorialText "They'll cause more damage to your ship ...")
            (Utilities|FlowControl|Delay 5.0)
            (Variables|Default|SettutorialText "Survive throughout the music track to advance to a next level ...")
            (Utilities|FlowControl|Delay 7.0)
            (Variables|Default|SettutorialText "Each level will be harder than the previous one ...")
            (Utilities|FlowControl|Delay 6.0)
            (Variables|Default|SettutorialText "Have fun and thanks for downloading Beat Rush!")
            (Utilities|FlowControl|Delay 5.0)
            (Variables|Default|SettutorialText ""))
          (:then_2
            (Variables|Default|SetmoveUpMultiplier 2.0)))
        (else
          ;[0 0.617 1 1 85] Level 2
          (if (or (== (Variables|Default|GetlevelNum) 2.0) (Variables|Default|GetisReplaying))
            (Audio|Components|Audio|SetSound _music_3 "/Game/audio/OST/ecstatic.ecstatic")
            (Audio|Components|Audio|Play _music_3 0.0)
            (Utilities|FlowControl|Delay 197.0)
            (Audio|PlaySound2D "/Game/audio/SFX/sfx2/sfx2/accomplished2.accomplished2" 1.0 1.0 0.0 0 0)
            (Utilities|FlowControl|Delay 1.0)
            (|ShowInterstitial
              (:then
                (if (== (Variables|Default|GetlevelNum) 2.0)
                  (bind _output_get_3 (Variables|Default|SetlevelNum 3.0))
                  (bind _success__2 (CallFunction|SaveALL (Variables|Default|GetsimtoonPointsNum) _output_get_3 (Variables|Default|GetcurrentShip) (Variables|Default|Getads_removed)))
                  (if _success__2
                    (Audio|PlaySound2D "/Game/audio/SFX/sfx2/sfx2/accomplished3.accomplished3" 1.0 1.0 0.0 0 0)
                    (Utilities|FlowControl|Delay 0.2)
                    (Transformation|SetActorLocationAndRotation "154.399994,36.360001,3547.199951" "0, 0,-179.800003" false true)
                    (goto _label_5)))))
            (else
              ;[0 1 0.7397 1 85] Level 3
              (if (or (== (Variables|Default|GetlevelNum) 3.0) (Variables|Default|GetisReplaying))
                (Audio|Components|Audio|SetSound _music_4 "/Game/audio/OST/greatMoments.greatMoments")
                (Audio|Components|Audio|Play _music_4 0.0)
                (Utilities|FlowControl|Delay 184.0)
                (Audio|PlaySound2D "/Game/audio/SFX/sfx2/sfx2/accomplished2.accomplished2" 1.0 1.0 0.0 0 0)
                (Utilities|FlowControl|Delay 1.0)
                (|ShowInterstitial
                  (:then
                    (if (== (Variables|Default|GetlevelNum) 3.0)
                      (bind _output_get_4 (Variables|Default|SetlevelNum 4.0))
                      (bind _success__3 (CallFunction|SaveALL (Variables|Default|GetsimtoonPointsNum) _output_get_4 (Variables|Default|GetcurrentShip) (Variables|Default|Getads_removed)))
                      (if _success__3
                        (Audio|PlaySound2D "/Game/audio/SFX/sfx2/sfx2/accomplished3.accomplished3" 1.0 1.0 0.0 0 0)
                        (Utilities|FlowControl|Delay 0.2)
                        (Transformation|SetActorLocationAndRotation "154.399994,36.360001,3547.199951" "0, 0,-179.800003" false true)
                        (goto _label_5)))))
                (else
                  ;[0 1 0.2921 1 85] Level 4
                  (if (or (== (Variables|Default|GetlevelNum) 4.0) (Variables|Default|GetisReplaying))
                    (Audio|Components|Audio|SetSound _music_5 "/Game/audio/OST/virus.virus")
                    (Audio|Components|Audio|Play _music_5 0.0)
                    (Utilities|FlowControl|Delay 195.0)
                    (Audio|PlaySound2D "/Game/audio/SFX/sfx2/sfx2/accomplished2.accomplished2" 1.0 1.0 0.0 0 0)
                    (Utilities|FlowControl|Delay 1.0)
                    (|ShowInterstitial
                      (:then
                        (if (== (Variables|Default|GetlevelNum) 4.0)
                          (bind _output_get_5 (Variables|Default|SetlevelNum 5.0))
                          (bind _success__4 (CallFunction|SaveALL (Variables|Default|GetsimtoonPointsNum) _output_get_5 (Variables|Default|GetcurrentShip) (Variables|Default|Getads_removed)))
                          (if _success__4
                            (Audio|PlaySound2D "/Game/audio/SFX/sfx2/sfx2/accomplished3.accomplished3" 1.0 1.0 0.0 0 0)
                            (Utilities|FlowControl|Delay 0.2)
                            (Transformation|SetActorLocationAndRotation "154.399994,36.360001,3547.199951" "0, 0,-179.800003" false true)
                            (goto _label_5)))))
                    (else
                      ;[0 0.4213 1 1 85] Level 5
                      (if (or (== (Variables|Default|GetlevelNum) 5.0) (Variables|Default|GetisReplaying))
                        (Audio|Components|Audio|SetSound _music_6 "/Game/audio/OST/poison.poison")
                        (Audio|Components|Audio|Play _music_6 0.0)
                        (Utilities|FlowControl|Delay 248.0)
                        (Audio|PlaySound2D "/Game/audio/SFX/sfx2/sfx2/accomplished2.accomplished2" 1.0 1.0 0.0 0 0)
                        (Utilities|FlowControl|Delay 1.0)
                        (|ShowInterstitial
                          (:then
                            (if (== (Variables|Default|GetlevelNum) 5.0)
                              (bind _output_get_6 (Variables|Default|SetlevelNum 6.0))
                              (bind _success__5 (CallFunction|SaveALL (Variables|Default|GetsimtoonPointsNum) _output_get_6 (Variables|Default|GetcurrentShip) (Variables|Default|Getads_removed)))
                              (if _success__5
                                (Audio|PlaySound2D "/Game/audio/SFX/sfx2/sfx2/accomplished3.accomplished3" 1.0 1.0 0.0 0 0)
                                (Utilities|FlowControl|Delay 0.2)
                                (Transformation|SetActorLocationAndRotation "154.399994,36.360001,3547.199951" "0, 0,-179.800003" false true)
                                (goto _label_5)))))
                        (else
                          ;[0 0 1 1 85] Level 6
                          (if (or (== (Variables|Default|GetlevelNum) 6.0) (Variables|Default|GetisReplaying))
                            (Audio|Components|Audio|SetSound _music_7 "/Game/audio/OST/animals.animals")
                            (Audio|Components|Audio|Play _music_7 0.0)
                            (Utilities|FlowControl|Delay 305.0)
                            (Audio|PlaySound2D "/Game/audio/SFX/sfx2/sfx2/accomplished2.accomplished2" 1.0 1.0 0.0 0 0)
                            (Utilities|FlowControl|Delay 1.0)
                            (|ShowInterstitial
                              (:then
                                (if (== (Variables|Default|GetlevelNum) 6.0)
                                  (bind _output_get_7 (Variables|Default|SetlevelNum 7.0))
                                  (bind _success__6 (CallFunction|SaveALL (Variables|Default|GetsimtoonPointsNum) _output_get_7 (Variables|Default|GetcurrentShip) (Variables|Default|Getads_removed)))
                                  (if _success__6
                                    (Audio|PlaySound2D "/Game/audio/SFX/sfx2/sfx2/accomplished3.accomplished3" 1.0 1.0 0.0 0 0)
                                    (Utilities|FlowControl|Delay 0.2)
                                    (Transformation|SetActorLocationAndRotation "154.399994,36.360001,3547.199951" "0, 0,-179.800003" false true)
                                    (goto _label_5)))))
                            (else
                              ;[1 0.8654 0 1 85] Level 7
                              (if (or (== (Variables|Default|GetlevelNum) 7.0) (Variables|Default|GetisReplaying))
                                (Audio|Components|Audio|SetSound _music "/Game/audio/OST/animals.animals")
                                (Audio|Components|Audio|Play _music 0.0)
                                (Utilities|FlowControl|Delay 305.0)
                                (Audio|PlaySound2D "/Game/audio/SFX/sfx2/sfx2/accomplished2.accomplished2" 1.0 1.0 0.0 0 0)
                                (Utilities|FlowControl|Delay 1.0)
                                (|ShowInterstitial
                                  (:then
                                    (if (== (Variables|Default|GetlevelNum) 7.0)
                                      (bind _output_get_8 (Variables|Default|SetlevelNum 8.0))
                                      (bind _success__7 (CallFunction|SaveALL (Variables|Default|GetsimtoonPointsNum) _output_get_8 (Variables|Default|GetcurrentShip) (Variables|Default|Getads_removed)))
                                      (if _success__7
                                        (Audio|PlaySound2D "/Game/audio/SFX/sfx2/sfx2/accomplished3.accomplished3" 1.0 1.0 0.0 0 0)
                                        (Utilities|FlowControl|Delay 0.2)
                                        (Transformation|SetActorLocationAndRotation "154.399994,36.360001,3547.199951" "0, 0,-179.800003" false true)))))))))))))))))))
    (:then_3
      (if (== (Variables|Default|GetlevelNum) 5.0)
        (if (Math|Random|RandomBool)
          (if (Math|Random|RandomBool)
            (Utilities|FlowControl|Delay 15.0)
            (Game|SetGamePaused true)
            (Utilities|FlowControl|DoOnce false
              (:Completed
                (|InAppPurchase (Game|GetPlayerController 0) (Utilities|Struct|MakeInAppPurchaseProductRequest "tokenofsupport" false)
                  (:OnSuccess
                    (Game|SetGamePaused false))
                  (:OnFailure
                    (Game|SetGamePaused false)))))))))))

(event Custom|respawnPlayer
  (Transformation|SetActorLocationAndRotation "35065.113281,-809.449280,439.583984" "0, 0,-179.800003" false true))

(event Custom|setShip
  (params (shipNum :type Float%20%28single-precision%29))
  (bind _staticmesh (Variables|Default|GetStaticMesh))
  (bind _cylinder (Variables|Default|GetCylinder))
  (bind _relativelocation (Variables|/Script/Engine.SceneComponent|GetRelativeLocation _staticmesh))
  (bind _returnvalue (- (.x _relativelocation) 1e+02))
  (if (== shipNum 2.0)
    (Components|StaticMesh|SetStaticMesh _staticmesh "/Game/Meshes/vessel/ship_2.ship_2")
    (Transformation|SetWorldScale3D _staticmesh "1.500000,1.500000,1.500000")
    (Transformation|SetWorldRotation _staticmesh "0, 0, 0" false false)
    (Transformation|SetRelativeLocation _staticmesh (Math|Vector|MakeVector _returnvalue 0.0 0.0) false false)
    (Components|DestroyComponent _cylinder)
    (Variables|Default|SetmaxHealth 3e+02)
    (elif (== shipNum 3.0)
      (Components|StaticMesh|SetStaticMesh _staticmesh "/Game/Meshes/vessel/ship_3.ship_3")
      (Transformation|SetWorldScale3D _staticmesh "0.500000,0.500000,0.500000")
      (Transformation|SetWorldRotation _staticmesh "0,90.000000, 0" false false)
      (Transformation|SetRelativeLocation _staticmesh (Math|Vector|MakeVector _returnvalue 0.0 0.0) false false)
      (Components|DestroyComponent _cylinder)
      (Variables|Default|SetmaxHealth 6.5e+02)
      (elif (== shipNum 4.0)
        (Components|StaticMesh|SetStaticMesh _staticmesh "/Game/Meshes/vessel/ship_4.ship_4")
        (Transformation|SetWorldScale3D _staticmesh "1.750000,1.750000,1.750000")
        (Transformation|SetWorldRotation _staticmesh "0,90.000000, 0" false false)
        (Transformation|SetRelativeLocation _staticmesh (Math|Vector|MakeVector _returnvalue 0.0 0.0) false false)
        (Components|DestroyComponent _cylinder)
        (Variables|Default|SetmaxHealth 1e+03)))))

(event Custom|applyDamage
  (params (howMuch :type Float%20%28single-precision%29))
  (Audio|PlaySound2D "/Game/audio/SFX/sfx2/sfx2/death1.death1" 1.0 1.0 0.0 0 0)
  (Variables|Default|Sethealth (- (Variables|Default|Gethealth) howMuch))
  (if (<= (Variables|Default|Gethealth) 0.0)
    (Game|SetGamePaused true)
    (Widget|RemovefromParent (stale Custom|startGame _returnvalue_21))
    (bind _returnvalue (UserInterface|CreateWidget "/Game/UI/deathScreen.deathScreen_C"))
    (UserInterface|Viewport|AddtoViewport _returnvalue 0)))

(event Custom|replayLevel
  (params (levelToReplay :type Integer))
  (bind _music (Variables|Default|Getmusic))
  (bind _music_2 (Variables|Default|Getmusic))
  (bind _music_3 (Variables|Default|Getmusic))
  (bind _music_4 (Variables|Default|Getmusic))
  (bind _music_5 (Variables|Default|Getmusic))
  (bind _music_6 (Variables|Default|Getmusic))
  (bind _music_7 (Variables|Default|Getmusic))
  (Variables|Default|SetisReplaying true)
  (switch int levelToReplay
    (:1
      ;[0 0.957 1 1 85] Level 1
      (if (or (== (Variables|Default|GetlevelNum) 1.0) (Variables|Default|GetisReplaying)) :!label _label
        (Audio|Components|Audio|SetSound _music_2 "/Game/audio/OST/caffeine.caffeine")
        (Utilities|FlowControl|Sequence
          (:then_0
            (Audio|Components|Audio|Play _music_2 0.0)
            (Utilities|FlowControl|Delay 1.5e+02)
            (Audio|PlaySound2D "/Game/audio/SFX/sfx2/sfx2/accomplished2.accomplished2" 1.0 1.0 0.0 0 0)
            (Utilities|FlowControl|Delay 1.0)
            (|ShowInterstitial
              (:then
                (if (== (Variables|Default|GetlevelNum) 1.0)
                  (bind _output_get (Variables|Default|SetlevelNum 2.0))
                  (bind _success_ (CallFunction|SaveALL (Variables|Default|GetsimtoonPointsNum) _output_get (Variables|Default|GetcurrentShip) (Variables|Default|Getads_removed)))
                  (if _success_
                    (Audio|PlaySound2D "/Game/audio/SFX/sfx2/sfx2/accomplished3.accomplished3" 1.0 1.0 0.0 0 0)
                    (Utilities|FlowControl|Delay 0.2)
                    (Variables|Default|SetmoveUpMultiplier 1.0)
                    (Transformation|SetActorLocationAndRotation "154.399994,36.360001,3547.199951" "0, 0,-179.800003" false true)
                    (goto _label))))))
          (:then_1
            (Utilities|FlowControl|Delay 3.0)
            (Variables|Default|SettutorialText "Welcome!")
            (Utilities|FlowControl|Delay 2.0)
            (Variables|Default|SettutorialText "Let's keep this simple ...")
            (Utilities|FlowControl|Delay 3.0)
            (Variables|Default|SettutorialText "Those colorful shining objects are what we call 'points' ...")
            (Utilities|FlowControl|Delay 5.0)
            (Variables|Default|SettutorialText "The blue ones serve as a digital currency within the game and restore your health")
            (Utilities|FlowControl|Delay 6.0)
            (Variables|Default|SettutorialText "You can buy stuff in the Shop with them ...")
            (Utilities|FlowControl|Delay 4.0)
            (Variables|Default|SettutorialText "The other ones only restore your health")
            (Utilities|FlowControl|Delay 4.0)
            (Variables|Default|SettutorialText "The rocks you see generating ahead are obstacles ...")
            (Utilities|FlowControl|Delay 4.0)
            (Variables|Default|SettutorialText "Avoid them to survive ...")
            (Utilities|FlowControl|Delay 3.5)
            (Variables|Default|SettutorialText "Later in the game, more obstacles will begin to appear ...")
            (Utilities|FlowControl|Delay 5.0)
            (Variables|Default|SettutorialText "They'll cause more damage to your ship ...")
            (Utilities|FlowControl|Delay 5.0)
            (Variables|Default|SettutorialText "Survive throughout the music track to advance to a next level ...")
            (Utilities|FlowControl|Delay 7.0)
            (Variables|Default|SettutorialText "Each level will be harder than the previous one ...")
            (Utilities|FlowControl|Delay 6.0)
            (Variables|Default|SettutorialText "Have fun and thanks for downloading Beat Rush!")
            (Utilities|FlowControl|Delay 5.0)
            (Variables|Default|SettutorialText ""))
          (:then_2
            (Variables|Default|SetmoveUpMultiplier 2.0)))
        (else
          ;[0 0.617 1 1 85] Level 2
          (if (or (== (Variables|Default|GetlevelNum) 2.0) (Variables|Default|GetisReplaying)) :!label _label_2
            (Audio|Components|Audio|SetSound _music_3 "/Game/audio/OST/ecstatic.ecstatic")
            (Audio|Components|Audio|Play _music_3 0.0)
            (Utilities|FlowControl|Delay 197.0)
            (Audio|PlaySound2D "/Game/audio/SFX/sfx2/sfx2/accomplished2.accomplished2" 1.0 1.0 0.0 0 0)
            (Utilities|FlowControl|Delay 1.0)
            (|ShowInterstitial
              (:then
                (if (== (Variables|Default|GetlevelNum) 2.0)
                  (bind _output_get_2 (Variables|Default|SetlevelNum 3.0))
                  (bind _success__2 (CallFunction|SaveALL (Variables|Default|GetsimtoonPointsNum) _output_get_2 (Variables|Default|GetcurrentShip) (Variables|Default|Getads_removed)))
                  (if _success__2
                    (Audio|PlaySound2D "/Game/audio/SFX/sfx2/sfx2/accomplished3.accomplished3" 1.0 1.0 0.0 0 0)
                    (Utilities|FlowControl|Delay 0.2)
                    (Transformation|SetActorLocationAndRotation "154.399994,36.360001,3547.199951" "0, 0,-179.800003" false true)
                    (goto _label)))))
            (else
              ;[0 1 0.7397 1 85] Level 3
              (if (or (== (Variables|Default|GetlevelNum) 3.0) (Variables|Default|GetisReplaying)) :!label _label_3
                (Audio|Components|Audio|SetSound _music_4 "/Game/audio/OST/greatMoments.greatMoments")
                (Audio|Components|Audio|Play _music_4 0.0)
                (Utilities|FlowControl|Delay 184.0)
                (Audio|PlaySound2D "/Game/audio/SFX/sfx2/sfx2/accomplished2.accomplished2" 1.0 1.0 0.0 0 0)
                (Utilities|FlowControl|Delay 1.0)
                (|ShowInterstitial
                  (:then
                    (if (== (Variables|Default|GetlevelNum) 3.0)
                      (bind _output_get_3 (Variables|Default|SetlevelNum 4.0))
                      (bind _success__3 (CallFunction|SaveALL (Variables|Default|GetsimtoonPointsNum) _output_get_3 (Variables|Default|GetcurrentShip) (Variables|Default|Getads_removed)))
                      (if _success__3
                        (Audio|PlaySound2D "/Game/audio/SFX/sfx2/sfx2/accomplished3.accomplished3" 1.0 1.0 0.0 0 0)
                        (Utilities|FlowControl|Delay 0.2)
                        (Transformation|SetActorLocationAndRotation "154.399994,36.360001,3547.199951" "0, 0,-179.800003" false true)
                        (goto _label)))))
                (else
                  ;[0 1 0.2921 1 85] Level 4
                  (if (or (== (Variables|Default|GetlevelNum) 4.0) (Variables|Default|GetisReplaying)) :!label _label_4
                    (Audio|Components|Audio|SetSound _music_5 "/Game/audio/OST/virus.virus")
                    (Audio|Components|Audio|Play _music_5 0.0)
                    (Utilities|FlowControl|Delay 195.0)
                    (Audio|PlaySound2D "/Game/audio/SFX/sfx2/sfx2/accomplished2.accomplished2" 1.0 1.0 0.0 0 0)
                    (Utilities|FlowControl|Delay 1.0)
                    (|ShowInterstitial
                      (:then
                        (if (== (Variables|Default|GetlevelNum) 4.0)
                          (bind _output_get_4 (Variables|Default|SetlevelNum 5.0))
                          (bind _success__4 (CallFunction|SaveALL (Variables|Default|GetsimtoonPointsNum) _output_get_4 (Variables|Default|GetcurrentShip) (Variables|Default|Getads_removed)))
                          (if _success__4
                            (Audio|PlaySound2D "/Game/audio/SFX/sfx2/sfx2/accomplished3.accomplished3" 1.0 1.0 0.0 0 0)
                            (Utilities|FlowControl|Delay 0.2)
                            (Transformation|SetActorLocationAndRotation "154.399994,36.360001,3547.199951" "0, 0,-179.800003" false true)
                            (goto _label)))))
                    (else
                      ;[0 0.4213 1 1 85] Level 5
                      (if (or (== (Variables|Default|GetlevelNum) 5.0) (Variables|Default|GetisReplaying)) :!label _label_5
                        (Audio|Components|Audio|SetSound _music_6 "/Game/audio/OST/poison.poison")
                        (Audio|Components|Audio|Play _music_6 0.0)
                        (Utilities|FlowControl|Delay 248.0)
                        (Audio|PlaySound2D "/Game/audio/SFX/sfx2/sfx2/accomplished2.accomplished2" 1.0 1.0 0.0 0 0)
                        (Utilities|FlowControl|Delay 1.0)
                        (|ShowInterstitial
                          (:then
                            (if (== (Variables|Default|GetlevelNum) 5.0)
                              (bind _output_get_5 (Variables|Default|SetlevelNum 6.0))
                              (bind _success__5 (CallFunction|SaveALL (Variables|Default|GetsimtoonPointsNum) _output_get_5 (Variables|Default|GetcurrentShip) (Variables|Default|Getads_removed)))
                              (if _success__5
                                (Audio|PlaySound2D "/Game/audio/SFX/sfx2/sfx2/accomplished3.accomplished3" 1.0 1.0 0.0 0 0)
                                (Utilities|FlowControl|Delay 0.2)
                                (Transformation|SetActorLocationAndRotation "154.399994,36.360001,3547.199951" "0, 0,-179.800003" false true)
                                (goto _label)))))
                        (else
                          ;[0 0 1 1 85] Level 6
                          (if (or (== (Variables|Default|GetlevelNum) 6.0) (Variables|Default|GetisReplaying)) :!label _label_6
                            (Audio|Components|Audio|SetSound _music_7 "/Game/audio/OST/animals.animals")
                            (Audio|Components|Audio|Play _music_7 0.0)
                            (Utilities|FlowControl|Delay 305.0)
                            (Audio|PlaySound2D "/Game/audio/SFX/sfx2/sfx2/accomplished2.accomplished2" 1.0 1.0 0.0 0 0)
                            (Utilities|FlowControl|Delay 1.0)
                            (|ShowInterstitial
                              (:then
                                (if (== (Variables|Default|GetlevelNum) 6.0)
                                  (bind _output_get_6 (Variables|Default|SetlevelNum 7.0))
                                  (bind _success__6 (CallFunction|SaveALL (Variables|Default|GetsimtoonPointsNum) _output_get_6 (Variables|Default|GetcurrentShip) (Variables|Default|Getads_removed)))
                                  (if _success__6
                                    (Audio|PlaySound2D "/Game/audio/SFX/sfx2/sfx2/accomplished3.accomplished3" 1.0 1.0 0.0 0 0)
                                    (Utilities|FlowControl|Delay 0.2)
                                    (Transformation|SetActorLocationAndRotation "154.399994,36.360001,3547.199951" "0, 0,-179.800003" false true)
                                    (goto _label)))))
                            (else
                              ;[1 0.8654 0 1 85] Level 7
                              (if (or (== (Variables|Default|GetlevelNum) 7.0) (Variables|Default|GetisReplaying))
                                (Audio|Components|Audio|SetSound _music "/Game/audio/OST/animals.animals")
                                (Audio|Components|Audio|Play _music 0.0)
                                (Utilities|FlowControl|Delay 305.0)
                                (Audio|PlaySound2D "/Game/audio/SFX/sfx2/sfx2/accomplished2.accomplished2" 1.0 1.0 0.0 0 0)
                                (Utilities|FlowControl|Delay 1.0)
                                (|ShowInterstitial
                                  (:then
                                    (if (== (Variables|Default|GetlevelNum) 7.0)
                                      (bind _output_get_7 (Variables|Default|SetlevelNum 8.0))
                                      (bind _success__7 (CallFunction|SaveALL (Variables|Default|GetsimtoonPointsNum) _output_get_7 (Variables|Default|GetcurrentShip) (Variables|Default|Getads_removed)))
                                      (if _success__7
                                        (Audio|PlaySound2D "/Game/audio/SFX/sfx2/sfx2/accomplished3.accomplished3" 1.0 1.0 0.0 0 0)
                                        (Utilities|FlowControl|Delay 0.2)
                                        (Transformation|SetActorLocationAndRotation "154.399994,36.360001,3547.199951" "0, 0,-179.800003" false true)))))))))))))))))))
    (:2
      (goto _label_2))
    (:3
      (goto _label_3))
    (:4
      (goto _label_4))
    (:5
      (goto _label_5))
    (:6
      (goto _label_6))))

(event Custom|clearPoints_obstacles
  (Utilities|FlowControl|Sequence
    (:then_0
      (for _array_element (Variables|Default|GetregularPointsArr)
        (Actor|DestroyActor _array_element)))
    (:then_1
      (for _array_element_2 (Variables|Default|GetbetterPointsArr)
        (Actor|DestroyActor _array_element_2)))
    (:then_2
      (for _array_element_3 (Variables|Default|GetsimtoonPointsArr)
        (Actor|DestroyActor _array_element_3)))
    (:then_3
      (for _array_element_4 (Variables|Default|GetobstacleV1Arr)
        (Actor|DestroyActor _array_element_4)))
    (:then_4
      (for _array_element_5 (Variables|Default|GetobstacleV2Arr)
        (Actor|DestroyActor _array_element_5)))
    (:then_5
      (for _array_element_6 (Variables|Default|GetobstacleV3Arr)
        (Actor|DestroyActor _array_element_6)))))

(event EventBeginPlay
  (bind _returnvalue (SaveGame|DoesSaveGameExist "main"))
  (if _returnvalue
    (CallFunction|RespawnPlayer)
    (bind _returnvalue_2 (SaveGame|LoadGamefromSlot "main"))
    (Utilities|IsValid _returnvalue_2
      (:Is%20Valid
        (Audio|PlaySound2D "/Game/audio/SFX/sfx2/sfx2/accomplished1.accomplished1" 1.0 1.0 0.0 0 0)
        (bind _output_get (Variables|Default|SetprimaryLoadObj _returnvalue_2))
        (bind _asprimary_save_obj (Utilities|Casting|CastToprimarySaveObj _output_get))
        (Variables|Default|SetlevelNum (Variables|/Game/primarySaveObj.primarySaveObj_C|GetlevelNumSave _asprimary_save_obj))
        (Variables|Default|SetsimtoonPointsNum (Variables|/Game/primarySaveObj.primarySaveObj_C|GettotalBluePointsSAVE _asprimary_save_obj))
        (CallFunction|SetShip (Variables|/Game/primarySaveObj.primarySaveObj_C|GetcurrentShipSAVE _asprimary_save_obj))
        (Variables|Default|Setads_removed (Variables|/Game/primarySaveObj.primarySaveObj_C|Getads_removedSAVE _asprimary_save_obj)))
      (:Is%20Not%20Valid
        (Audio|PlaySound2D "/Game/audio/SFX/sfx2/sfx2/death2.death2" 1.0 1.0 0.0 0 0)
        (bind _returnvalue_3 (SaveGame|CreateSaveGameObject "/Game/primarySaveObj.primarySaveObj_C" :!label _label))
        (Variables|Default|SetprimarySaveObj _returnvalue_3)))
    (else
      (Audio|PlaySound2D "/Game/audio/SFX/sfx2/sfx2/crash.crash" 1.0 1.0 0.0 0 0)
      (goto _label)))
  (bind _returnvalue_4 (UserInterface|CreateWidget "/Game/UI/main_menu.main_menu_C"))
  (bind _output_get_2 (Variables|Default|SetmainMenu _returnvalue_4))
  (UserInterface|Viewport|AddtoViewport _output_get_2 0)
  (Variables|Default|SetpointsNum (+ (Variables|Default|GetregularPointsNum) (Variables|Default|GetsimtoonPointsNum) (Variables|Default|GetbetterPointsNum)))
  (for _array_element (Utilities|Array|MakeArray (Math|Transform|MakeTransform (Math|Vector|MakeVector (Math|Random|RandomFloatinRange 0.0 2.5e+04) (Math|Random|RandomFloatinRange 4e+03 1.2e+04) -1.5e+03) "0, 0, 0" "2.000000,2.000000,2.000000") (Math|Transform|MakeTransform (Math|Vector|MakeVector (Math|Random|RandomFloatinRange 0.0 2.5e+04) (Math|Random|RandomFloatinRange 4e+03 1.2e+04) -1.5e+03) "0, 0, 0" "2.000000,2.000000,2.000000") (Math|Transform|MakeTransform (Math|Vector|MakeVector (Math|Random|RandomFloatinRange 0.0 2.5e+04) (Math|Random|RandomFloatinRange 4e+03 1.2e+04) -1.5e+03) "0, 0, 0" "2.000000,2.000000,2.000000") (Math|Transform|MakeTransform (Math|Vector|MakeVector (Math|Random|RandomFloatinRange 0.0 2.5e+04) (Math|Random|RandomFloatinRange -1.5e+04 -6e+03) -1.5e+03) "0, 0, 0" "2.000000,2.000000,2.000000") (Math|Transform|MakeTransform (Math|Vector|MakeVector (Math|Random|RandomFloatinRange 0.0 2.5e+04) (Math|Random|RandomFloatinRange -1.5e+04 -6e+03) -1.5e+03) "0, 0, 0" "2.000000,2.000000,2.000000") (Math|Transform|MakeTransform (Math|Vector|MakeVector (Math|Random|RandomFloatinRange 0.0 2.5e+04) (Math|Random|RandomFloatinRange 4e+03 1.2e+04) -1.5e+03) "0, 0, 0" "2.000000,2.000000,2.000000") (Math|Transform|MakeTransform (Math|Vector|MakeVector (Math|Random|RandomFloatinRange 0.0 2.5e+04) (Math|Random|RandomFloatinRange -1.5e+04 -6e+03) -1.5e+03) "0, 0, 0" "2.000000,2.000000,2.000000")) :!label _label_2
    (Game|SpawnActorfromClass "/Game/BP/mountain_Blueprint.mountain_Blueprint_C" _array_element "AdjustIfPossibleButAlwaysSpawn" 0 0))
  (Utilities|FlowControl|Delay 15.0)
  (goto _label_2))

(event EventTick
  (params (DeltaSeconds :type Float%20%28single-precision%29))
  (bind _maxhealth (Variables|Default|GetmaxHealth))
  (Utilities|FlowControl|Sequence
    (:then_0
      (if (Variables|Default|GetisGameFocused)
        (Transformation|AddRelativeLocation (Variables|Collision|GetCapsuleComponent) (Math|Vector|MakeVector (+ (* (.x (+ (Math|Vector|MakeVector (.x (Math|Vector|NegateVector (Transformation|GetActorForwardVector))) 0.0 0.0) 0.0)) 6e+01 (Variables|Default|GetlevelNum) (Variables|Default|GetmoveUpMultiplier)) (* (Variables|Default|GetlevelNum) (* (* (stale Input|AxisEvents|InputAxisMoveUp AxisValue) -1.0) 15.0))) 0.0 0.0) false false)))
    (:then_1
      (if (>= (Variables|Default|Gethealth) _maxhealth)
        (Variables|Default|Sethealth _maxhealth)))))

(event Input|AxisEvents|InputAxisMoveRight
  (params (AxisValue :type Float%20%28single-precision%29))
  (bind _returnvalue (* AxisValue 17.0))
  (bind _staticmesh (Variables|Default|GetStaticMesh))
  (bind _relativerotation (Variables|/Script/Engine.SceneComponent|GetRelativeRotation _staticmesh))
  (Transformation|AddRelativeLocation (Variables|Collision|GetCapsuleComponent) (Math|Vector|MakeVector 0.0 (* (* AxisValue -1.0) 5e+01) 0.0) false false)
  (if (== (Variables|Default|GetcurrentShip) 1.0)
    (Transformation|SetRelativeRotation _staticmesh (Math|Rotator|MakeRotator (.roll _relativerotation) _returnvalue (.yaw _relativerotation)) false false)
    (else
      (Transformation|SetRelativeRotation _staticmesh (Math|Rotator|MakeRotator (.roll _relativerotation) (* _returnvalue -1.0) (.yaw _relativerotation)) false false))))

(event Input|AxisEvents|InputAxisMoveUp
  (params (AxisValue :type Float%20%28single-precision%29)))

(event Input|KeyboardEvents|V
  (params (Key :type Key%20Structure :default "None"))
  (bind _staticmesh (Variables|Default|GetStaticMesh))
  (:Pressed
    (Components|StaticMesh|SetStaticMesh _staticmesh "/Game/Meshes/vessel/ship_4.ship_4")
    (Transformation|SetWorldScale3D _staticmesh "1.750000,1.750000,1.750000")
    (Transformation|SetWorldRotation _staticmesh "0,90.000000, 0" false false)
    (Transformation|SetRelativeLocation _staticmesh (Math|Vector|MakeVector (- (.x (Variables|/Script/Engine.SceneComponent|GetRelativeLocation _staticmesh)) 1e+02) 0.0 0.0) false false)
    (Components|DestroyComponent (Variables|Default|GetCylinder))
    (Variables|Default|SetmaxHealth 1e+03)))

(event Input|KeyboardEvents|G
  (params (Key :type Key%20Structure :default "None"))
  (:Pressed
    (Variables|Default|SetcurrentShip 4.0)
    (CallFunction|SetShip 4.0)))

(fn ConstructionScript)

(fn SaveALL
  (params (totalBluePoints :type Integer) (levelNum :type Float%20%28single-precision%29) (currentShip :type Float%20%28single-precision%29) (ads_removed :type Boolean))
  (Class|AndroidPermissionFunctionLibrary|AcquirePermissions (Utilities|Array|MakeArray "WRITE_EXTERNAL_STORAGE"))
  (bind _returnvalue (SaveGame|CreateSaveGameObject "/Game/primarySaveObj.primarySaveObj_C"))
  (Variables|Default|SetprimarySaveObj _returnvalue)
  (Variables|/Game/primarySaveObj.primarySaveObj_C|SetlevelNumSave (Variables|Default|GetprimarySaveObj) levelNum)
  (Variables|/Game/primarySaveObj.primarySaveObj_C|SettotalBluePointsSAVE (Variables|Default|GetprimarySaveObj) totalBluePoints)
  (Variables|/Game/primarySaveObj.primarySaveObj_C|SetcurrentShipSAVE (Variables|Default|GetprimarySaveObj) currentShip)
  (Variables|/Game/primarySaveObj.primarySaveObj_C|Setads_removedSAVE (Variables|Default|GetprimarySaveObj) ads_removed)
  (bind _returnvalue_2 (SaveGame|SaveGametoSlot (Variables|Default|GetprimarySaveObj) "main"))
  (return _returnvalue_2))

(fn ReloadALL
  (bind _asprimary_save_obj (Utilities|Casting|CastToprimarySaveObj (Variables|Default|GetprimaryLoadObj)))
  (Variables|Default|Setads_removed (Variables|/Game/primarySaveObj.primarySaveObj_C|Getads_removedSAVE _asprimary_save_obj))
  (Variables|Default|SetcurrentShip (Variables|/Game/primarySaveObj.primarySaveObj_C|GetcurrentShipSAVE _asprimary_save_obj))
  (Variables|Default|SetlevelNum (Variables|/Game/primarySaveObj.primarySaveObj_C|GetlevelNumSave _asprimary_save_obj))
  (Variables|Default|SetsimtoonPointsNum (Variables|/Game/primarySaveObj.primarySaveObj_C|GettotalBluePointsSAVE _asprimary_save_obj))
  (return true))