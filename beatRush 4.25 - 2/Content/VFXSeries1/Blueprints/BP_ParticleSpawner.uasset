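; BP_ParticleSpawner is an actor that continuously spawns BP_BaseProjectile actors at random points around itself, within a Spread range on each axis.
; A self-calling Loop event, started on BeginPlay, spawns a projectile every 0.2 seconds with the spawner's rotation and scale.
; Each projectile receives the configured type and particle template, plus impact and trail particles picked independently at random from arrays.
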(event Custom|Loop
  (bind _returnvalue (Transformation|GetActorTransform))
  (bind _resultparticles (Variables|Default|GetResultParticles))
  (bind _spread (Variables|Default|GetSpread))
  (bind _tailparticles (Variables|Default|GetTailParticles))
  (bind (_location _rotation _scale) (Math|Transform|BreakTransform _returnvalue))
  (bind _returnvalue_2 (* -1 _spread))
  (bind (_x _y _z) (Math|Vector|BreakVector _location))
  ;[1 1 1] Spawns particle based on transform selected
  (bind _returnvalue_3 (Game|SpawnActorfromClass "/Game/VFXSeries1/Blueprints/BP_BaseProjectile.BP_BaseProjectile_C" (Math|Transform|MakeTransform (Math|Vector|MakeVector (+ _x (Math|Random|RandomFloatinRange _returnvalue_2 _spread)) (+ _y (Math|Random|RandomFloatinRange _returnvalue_2 _spread)) (+ _z (Math|Random|RandomFloatinRange _returnvalue_2 _spread))) _rotation _scale) "Undefined" 0 "NewEnumerator0" 0))
  (Variables|/Game/VFXSeries1/Blueprints/BP_BaseProjectile.BP_BaseProjectile_C|SetProjectileType _returnvalue_3 (Variables|Default|GetProjectileType))
  ;[1 1 1] Sets particle templates for spawned projectile
  (Variables|/Game/VFXSeries1/Blueprints/BP_BaseProjectile.BP_BaseProjectile_C|SetImpactParticle _returnvalue_3 (Utilities|Array|Get(acopy) _resultparticles (Math|Random|RandomIntegerinRange 0 (Utilities|Array|LastIndex _resultparticles))))
  (Variables|/Game/VFXSeries1/Blueprints/BP_BaseProjectile.BP_BaseProjectile_C|SetTrailParticle _returnvalue_3 (Utilities|Array|Get(acopy) _tailparticles (Math|Random|RandomIntegerinRange 0 (Utilities|Array|LastIndex _tailparticles))))
  (Effects|Components|ParticleSystem|SetTemplate (Variables|/Game/VFXSeries1/Blueprints/BP_BaseProjectile.BP_BaseProjectile_C|GetPlasma/Kinetic%20particle _returnvalue_3) (Variables|Default|GetProjectileParticle))
  (Utilities|FlowControl|Delay 0.2)
  (CallFunction|Loop))

(event EventBeginPlay
  (bind _returnvalue (Transformation|GetActorTransform))
  (bind _resultparticles (Variables|Default|GetResultParticles))
  (bind _spread (Variables|Default|GetSpread))
  (bind _tailparticles (Variables|Default|GetTailParticles))
  (bind (_location _rotation _scale) (Math|Transform|BreakTransform _returnvalue))
  (bind _returnvalue_2 (* -1 _spread))
  (bind (_x _y _z) (Math|Vector|BreakVector _location))
  ;[1 1 1] Spawns particle based on transform selected
  (bind _returnvalue_3 (Game|SpawnActorfromClass "/Game/VFXSeries1/Blueprints/BP_BaseProjectile.BP_BaseProjectile_C" (Math|Transform|MakeTransform (Math|Vector|MakeVector (+ _x (Math|Random|RandomFloatinRange _returnvalue_2 _spread)) (+ _y (Math|Random|RandomFloatinRange _returnvalue_2 _spread)) (+ _z (Math|Random|RandomFloatinRange _returnvalue_2 _spread))) _rotation _scale) "Undefined" 0 "NewEnumerator0" 0))
  (Variables|/Game/VFXSeries1/Blueprints/BP_BaseProjectile.BP_BaseProjectile_C|SetProjectileType _returnvalue_3 (Variables|Default|GetProjectileType))
  ;[1 1 1] Sets particle templates for spawned projectile
  (Variables|/Game/VFXSeries1/Blueprints/BP_BaseProjectile.BP_BaseProjectile_C|SetImpactParticle _returnvalue_3 (Utilities|Array|Get(acopy) _resultparticles (Math|Random|RandomIntegerinRange 0 (Utilities|Array|LastIndex _resultparticles))))
  (Variables|/Game/VFXSeries1/Blueprints/BP_BaseProjectile.BP_BaseProjectile_C|SetTrailParticle _returnvalue_3 (Utilities|Array|Get(acopy) _tailparticles (Math|Random|RandomIntegerinRange 0 (Utilities|Array|LastIndex _tailparticles))))
  (Effects|Components|ParticleSystem|SetTemplate (Variables|/Game/VFXSeries1/Blueprints/BP_BaseProjectile.BP_BaseProjectile_C|GetPlasma/Kinetic%20particle _returnvalue_3) (Variables|Default|GetProjectileParticle))
  (Utilities|FlowControl|Delay 0.2)
  (CallFunction|Loop))

(fn ConstructionScript)