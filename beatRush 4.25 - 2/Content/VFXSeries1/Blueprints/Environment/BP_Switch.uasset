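; BP_Switch is a VFX showcase environment Blueprint that starts projectile simulation on a connected weapon test.
; On BeginPlay it enables the referenced WeaponTest, then casts that test's BPTarget child actor to BP_Target.
; It copies its PlayerEntered value into the target's BeginSimulation once, with no overlap or input handling in the graph.
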(event EventBeginPlay
  (bind _weapontest (Variables|Default|GetWeaponTest))
  (bind _bp_target (Variables|/Game/VFXSeries1/Blueprints/Environment/BP_WeaponTest.BP_WeaponTest_C|GetBP_Target _weapontest))
  (bind _childactor (Variables|/Script/Engine.ChildActorComponent|GetChildActor _bp_target))
  ;[1 1 1] Begins projectile simulation on connected weapon test
  (Utilities|IsValid (Variables|Default|GetWeaponTest)
    (:Is%20Valid
      (Variables|/Game/VFXSeries1/Blueprints/Environment/BP_WeaponTest.BP_WeaponTest_C|SetEnabled (Variables|Default|GetWeaponTest) true)
      (Utilities|IsValid _childactor
        (:Is%20Valid
          (bind _asbp_target (Utilities|Casting|CastToBP_Target _childactor))
          (Variables|/Game/VFXSeries1/Blueprints/Environment/BP_Target.BP_Target_C|SetBeginSimulation _asbp_target (Variables|Default|GetPlayerEntered)))))))

(fn ConstructionScript)