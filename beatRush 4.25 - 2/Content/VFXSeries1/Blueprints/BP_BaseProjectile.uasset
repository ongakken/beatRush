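; Base projectile actor for the VFX pack, with a type switch between moving plasma/kinetic shots and an instant beam, plus optional homing.
; Moving shots spawn a decal and impact particle on hit, then destroy themselves.
; Beam type zeroes movement on BeginPlay, line-traces forward against WorldStatic, stretches the beam particle to the impact and spawns effects there.
; Optional ricochet spawns a same-type projectile at the impact, oriented from the surface normal.
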(event Custom|DestroySelf
  ;[1 1 1] Destroys actor when called after minor delay
  (Utilities|FlowControl|Delay 0.2)
  (Actor|DestroyActor))

(event EventBeginPlay
  ;[1 1 1] When projectile is spawned, it runs a check to find what behavior is desired and then sets appropriate particle
  (Utilities|FlowControl|Delay 0.003)
  (CallFunction|CheckProjectileID)
  (Effects|Components|ParticleSystem|SetTemplate (Variables|Default|GetTail) (Variables|Default|GetTrailParticle)))

(event EventTick
  (params (DeltaSeconds :type Float%20%28single-precision%29))
  ;[1 1 1] Sets delta time
  (Variables|Default|SetDeltaTime DeltaSeconds))

(event Collision|EventHit
  (params (MyComp :type Primitive%20Component%20Object%20Reference) (Other :type Actor%20Object%20Reference) (OtherComp :type Primitive%20Component%20Object%20Reference) (bSelfMoved :type Boolean) (HitLocation :type Vector) (HitNormal :type Vector :default "0, 0, 0") (NormalImpulse :type Vector :default "0, 0, 0") (Hit :type Hit%20Result%20Structure%20%28by%20ref%29))
  (bind (_bblockinghit _binitialoverlap _time _location _impactpoint _normal _impactnormal) (Collision|BreakHitResult Hit))
  (bind _projectiletype (Variables|Default|GetProjectileType))
  (bind _returnvalue (Math|Conversions|RotationFromXVector _impactnormal))
  ;[1 1 1] On event hit the projectile will spawn a decal at the hit location using the set decal class
  (if (!= Other self)
    (bind _returnvalue_2 (Game|SpawnActorfromClass (Variables|VFX|GetDecalClass) (Math|Transform|MakeTransform _impactpoint _returnvalue (Variables|VFX|GetDecalSize)) "Undefined" 0 true 0))
    ;[1 1 1] Checks whether projectile is a energy based projectile such as beam or plasma and then spawns a particle at hit location
    (Variables|Default|SetImpactPoint _impactpoint)
    (Variables|Default|SetImpactNormal _impactnormal)
    (Variables|/Game/VFXSeries1/Blueprints/BP_BaseDecal.BP_BaseDecal_C|SetEnergy? _returnvalue_2 (or (Utilities|Enum|Equal(Enum) _projectiletype "NewEnumerator1") (Utilities|Enum|Equal(Enum) _projectiletype "NewEnumerator2")))
    (if (Utilities|Enum|NotEqual(Enum) (Variables|Default|GetProjectileType) "NewEnumerator2")
      (Effects|SpawnEmitteratLocation (Variables|VFX|GetImpactParticle) _impactpoint _returnvalue)
      ;[1 1 1] Sets the projectile visibility and then checks for whether ricohet is enabled before destroying actor
      (Rendering|SetVisibility (Variables|Default|GetPlasma/Kinetic%20particle) false false)
      (if (Variables|ProjectileSettings|GetRicochet)
        (CallFunction|HitRicochet))
      (Utilities|FlowControl|Delay 0.3)
      (Actor|DestroyActor))))

(fn ConstructionScript
  ;[1 1 1] Initializes homing system and sets template for trail particle then sets beam particle visibility
  (CallFunction|HomingSetup)
  (Effects|Components|ParticleSystem|SetTemplate (Variables|Default|GetTail) (Variables|Default|GetTrailParticle))
  (Rendering|Material|SetMaterial (Variables|Default|GetFlares) 0 0)
  (Rendering|SetVisibility (Variables|Default|GetBeamTypeParticle) false false))

(fn HomingSetup
  (bind _projectilemovement (Variables|Default|GetProjectileMovement))
  ;[1 1 1] Enables homing movement in the projectile movement component and then sets the target
  (Variables|/Script/Engine.ProjectileMovementComponent|SetbIsHomingProjectile _projectilemovement (Variables|ProjectileSettings|GetHoming))
  (Variables|/Script/Engine.ProjectileMovementComponent|SetHomingTargetComponent _projectilemovement (Variables|ProjectileSettings|GetHomingTarget)))

(fn CheckProjectileID
  (bind _returnvalue (Transformation|GetActorLocation))
  (bind _beamtypeparticle (Variables|Default|GetBeamTypeParticle))
  (bind _beamtypeparticle_2 (Variables|Default|GetBeamTypeParticle))
  (bind _projectiletype (Variables|Default|GetProjectileType))
  (bind _projectilemovement (Variables|Default|GetProjectileMovement))
  ;[1 1 1] Checks projectile preset and applies appropriate visibility
  (Utilities|FlowControl|Sequence
    (:then_0
      (if (Utilities|Enum|Equal(Enum) _projectiletype "NewEnumerator0")
        (Rendering|SetVisibility _beamtypeparticle_2 false false)))
    (:then_1
      (if (Utilities|Enum|Equal(Enum) _projectiletype "NewEnumerator1")
        (Rendering|SetVisibility _beamtypeparticle_2 false false)))
    (:then_2
      (if (Utilities|Enum|Equal(Enum) _projectiletype "NewEnumerator2")
        (Rendering|SetVisibility (Variables|Default|GetPlasma/Kinetic%20particle) false false)
        ;[1 1 1] Sets impact particle, negates all projectile velocity and speed then begins a line trace to establish beam behavour
        (Variables|VFX|SetImpactParticle "/Game/VFXSeries1/Particles/Energy/P_LaserImpact.P_LaserImpact")
        (Variables|/Script/Engine.ProjectileMovementComponent|SetInitialSpeed _projectilemovement 0.0)
        (Variables|/Script/Engine.ProjectileMovementComponent|SetMaxSpeed _projectilemovement 0.0)
        (Variables|/Script/Engine.MovementComponent|SetVelocity _projectilemovement "0, 0, 0")
        (bind _outhit (Collision|LineTraceForObjects _returnvalue (+ _returnvalue (* (Math|Rotator|GetRotationXVector (Transformation|GetActorRotation)) 5e+03)) (Utilities|Array|MakeArray "ObjectTypeQuery1") true (Variables|Default|GetReferenceArray) "None"))
        ;[1 1 1] Gets beam origin and line trace end, applies locations to the beam particle for beam source and target points
        (Class|ParticleSystemComponent|SetBeamSourcePoint _beamtypeparticle 0 _returnvalue)
        (Variables|Default|SetImpactPoint (.ImpactPoint (Collision|BreakHitResult _outhit)))
        (Variables|Default|SetImpactNormal (.ImpactNormal (Collision|BreakHitResult _outhit)))
        (Class|ParticleSystemComponent|SetBeamTargetPoint _beamtypeparticle 0 (Variables|Default|GetImpactPoint))
        ;[1 1 1] Set beam visibility, applies a particle and decal at beam endpoint
        (Rendering|SetVisibility (Variables|Default|GetBeamTypeParticle) true false)
        (Effects|SpawnEmitteratLocation (Variables|VFX|GetImpactParticle) (Variables|Default|GetImpactPoint))
        (Game|SpawnActorfromClass (Variables|VFX|GetDecalClass) (Math|Transform|MakeTransform (Variables|Default|GetImpactPoint) (Math|Conversions|RotationFromXVector (Variables|Default|GetImpactNormal)) (Variables|VFX|GetDecalSize)) "Undefined" 0 true 0)
        ;[1 1 1] Checks whether beam has ricochet and then destroys actor
        (if (Variables|ProjectileSettings|GetRicochet)
          (CallFunction|HitRicochet))
        (CallFunction|DestroySelf)))))

(fn HitRicochet
  (bind _impactnormal (Variables|Default|GetImpactNormal))
  (bind _returnvalue (Math|Conversions|RotationFromXVector _impactnormal))
  (bind (_roll _pitch _yaw) (Math|Rotator|BreakRotator _returnvalue))
  ;[1 1 1] If the projectile has ricochet enabled then this system will spawn a new projectile based upon the hit angle with the same characteristics as the previous projectile
  (bind _returnvalue_2 (Game|SpawnActorfromClass "BP_BaseProjectile_C" (Math|Transform|MakeTransform (Variables|Default|GetImpactPoint) (Math|Rotator|MakeRotator _roll (* _pitch 2.0) _yaw)) "Undefined" 0 (Variables|Default|GetProjectileType) 0))
  (Variables|BP_BaseProjectile_C|SetDecalSize _returnvalue_2 (Variables|VFX|GetDecalSize))
  (Variables|BP_BaseProjectile_C|SetImpactParticle _returnvalue_2 (Variables|VFX|GetImpactParticle))
  (Variables|BP_BaseProjectile_C|SetTrailParticle _returnvalue_2 (Variables|Default|GetTrailParticle)))