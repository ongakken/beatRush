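; Forcefield hit effect that shows an animated impact on a shielded static or skeletal mesh.
; OnImpact sets up the mesh, falling back to a capsule shape, and picks a simple, complex or instanced impact material from the shield's material or an override index, defaulting to complex.
; A dynamic instance fills the material slots while a timeline drives its HitPosition (mesh location plus hit offset) and Phase.
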(event EventOnImpact
  (params (Location :type Vector :default "0, 0, 0") (Mesh :type Static%20Mesh%20Component%20Object%20Reference) (Material :type Material%20Interface%20Object%20Reference) (MaterialOverwrite :type Integer) (SkeletalMesh :type Skeletal%20Mesh%20Component%20Object%20Reference))
  (bind _returnvalue (Rendering|Material|GetMaterials Mesh))
  (bind _returnvalue_2 (Rendering|Material|GetMaterials SkeletalMesh))
  (bind _returnvalue_3 (Utilities|Array|Length _returnvalue_2))
  (bind _returnvalue_4 (Utilities|Array|Length _returnvalue))
  (Utilities|IsValid SkeletalMesh
    (:Is%20Valid
      (Class|SkinnedMeshComponent|SetSkeletalMesh (Variables|Default|GetSkeletalMesh) (Variables|/Script/Engine.SkinnedMeshComponent|GetSkeletalMesh SkeletalMesh) true)
      ;[1 1 1] Find the used material and spawn a corresponding hit effect (or if overwrite is > 0 then use a specific effect for each number > 0)
      (if (== MaterialOverwrite 0)
        (if (== Material "/Game/ForcefieldSystem/Materials/ShieldMaterials/ff_Material_Simple.ff_Material_Simple")
          (bind _returnvalue_5 (Rendering|Material|CreateDynamicMaterialInstance 0 "/Game/ForcefieldSystem/Materials/ImpactMaterials/ff_Impact_SimpleMat.ff_Impact_SimpleMat" "None" :!class /Script/Engine.PrimitiveComponent :!label _label))
          (bind _output_get (Variables|Default|SetDynamicMaterial _returnvalue_5))
          (for _index (range 0 _returnvalue_3)
            (Rendering|Material|SetMaterial _index _output_get)
            (Rendering|Material|SetMaterial (Variables|Default|GetSkeletalMesh) _index _output_get))
          ;[1 1 1] Play the animation
          (bind _time (Timeline|Timeline_0 PlayFromStart)
            (:Update
              (Rendering|Material|SetVectorParameterValue (Variables|Default|GetDynamicMaterial) "HitPosition" (Math|Conversions|ToLinearColor(Vector) (+ (Transformation|GetWorldLocation SkeletalMesh) Location)) :!class /Script/Engine.MaterialInstanceDynamic)
              (Rendering|Material|SetScalarParameterValue (Variables|Default|GetDynamicMaterial) "Phase" _time :!class /Script/Engine.MaterialInstanceDynamic)))
          (elif (== Material "/Game/ForcefieldSystem/Materials/ShieldMaterials/ff_Material_Complex.ff_Material_Complex")
            (bind _returnvalue_6 (Rendering|Material|CreateDynamicMaterialInstance 0 "/Game/ForcefieldSystem/Materials/ImpactMaterials/ff_Impact_ComplexMat.ff_Impact_ComplexMat" "None" :!class /Script/Engine.PrimitiveComponent :!label _label_2))
            (bind _output_get_2 (Variables|Default|SetDynamicMaterial _returnvalue_6))
            (for _index_2 (range 0 _returnvalue_3)
              (Rendering|Material|SetMaterial _index_2 _output_get_2)
              (Rendering|Material|SetMaterial (Variables|Default|GetSkeletalMesh) _index_2 _output_get_2))
            (Timeline|Timeline_0 PlayFromStart)
            (elif (== Material "/Game/ForcefieldSystem/Materials/ShieldMaterials/ff_Material_tSimple_Inst.ff_Material_tSimple_Inst")
              (bind _returnvalue_7 (Rendering|Material|CreateDynamicMaterialInstance 0 "/Game/ForcefieldSystem/Materials/ImpactMaterials/ff_ImpactSimpleMat_Inst.ff_ImpactSimpleMat_Inst" "None" :!class /Script/Engine.PrimitiveComponent :!label _label_3))
              (bind _output_get_3 (Variables|Default|SetDynamicMaterial _returnvalue_7))
              (for _index_3 (range 0 _returnvalue_3)
                (Rendering|Material|SetMaterial _index_3 _output_get_3)
                (Rendering|Material|SetMaterial (Variables|Default|GetSkeletalMesh) _index_3 _output_get_3))
              (Timeline|Timeline_0 PlayFromStart)
              (else
                (goto _label_2)))))
        (else
          ;;[1 1 1] Overwrite Material
          (if (== MaterialOverwrite 1)
            (goto _label)
            (elif (== MaterialOverwrite 2)
              (goto _label_2)
              (elif (== MaterialOverwrite 3)
                (goto _label_3)
                (else
                  (goto _label_2))))))))
    (:Is%20Not%20Valid
      (Utilities|IsValid Mesh
        (:Is%20Valid
          (Components|StaticMesh|SetStaticMesh (Variables|/Script/Engine.StaticMeshComponent|GetStaticMesh Mesh)))
        (:Is%20Not%20Valid
          (Components|StaticMesh|SetStaticMesh "/Game/ForcefieldSystem/Meshes/Shape_NarrowCapsule.Shape_NarrowCapsule")))
      ;[1 1 1] Find the used material and spawn a corresponding hit effect (or if overwrite is > 0 then use a specific effect for each number > 0)
      (if (== MaterialOverwrite 0)
        (if (== Material "/Game/ForcefieldSystem/Materials/ShieldMaterials/ff_Material_Simple.ff_Material_Simple")
          (bind _returnvalue_8 (Rendering|Material|CreateDynamicMaterialInstance 0 "/Game/ForcefieldSystem/Materials/ImpactMaterials/ff_Impact_SimpleMat.ff_Impact_SimpleMat" "None" :!class /Script/Engine.PrimitiveComponent :!label _label_4))
          (bind _output_get_4 (Variables|Default|SetDynamicMaterial _returnvalue_8))
          (for _index_4 (range 0 _returnvalue_4)
            (Rendering|Material|SetMaterial _index_4 _output_get_4)
            (Rendering|Material|SetMaterial SkeletalMesh _index_4 _output_get_4))
          ;[1 1 1] Play the animation
          (bind _time_2 (Timeline|Timeline PlayFromStart)
            (:Update
              (Rendering|Material|SetVectorParameterValue (Variables|Default|GetDynamicMaterial) "HitPosition" (Math|Conversions|ToLinearColor(Vector) (+ (Transformation|GetWorldLocation Mesh) Location)) :!class /Script/Engine.MaterialInstanceDynamic)
              (Rendering|Material|SetScalarParameterValue (Variables|Default|GetDynamicMaterial) "Phase" _time_2 :!class /Script/Engine.MaterialInstanceDynamic)))
          (elif (== Material "/Game/ForcefieldSystem/Materials/ShieldMaterials/ff_Material_Complex.ff_Material_Complex")
            (bind _returnvalue_9 (Rendering|Material|CreateDynamicMaterialInstance 0 "/Game/ForcefieldSystem/Materials/ImpactMaterials/ff_Impact_ComplexMat.ff_Impact_ComplexMat" "None" :!class /Script/Engine.PrimitiveComponent :!label _label_5))
            (bind _output_get_5 (Variables|Default|SetDynamicMaterial _returnvalue_9))
            (for _index_5 (range 0 _returnvalue_4)
              (Rendering|Material|SetMaterial _index_5 _output_get_5)
              (Rendering|Material|SetMaterial (Variables|Default|GetSkeletalMesh) _index_5 _output_get_5))
            (Timeline|Timeline PlayFromStart)
            (elif (== Material "/Game/ForcefieldSystem/Materials/ShieldMaterials/ff_Material_tSimple_Inst.ff_Material_tSimple_Inst")
              (bind _returnvalue_10 (Rendering|Material|CreateDynamicMaterialInstance 0 "/Game/ForcefieldSystem/Materials/ImpactMaterials/ff_ImpactSimpleMat_Inst.ff_ImpactSimpleMat_Inst" "None" :!class /Script/Engine.PrimitiveComponent :!label _label_6))
              (bind _output_get_6 (Variables|Default|SetDynamicMaterial _returnvalue_10))
              (for _index_6 (range 0 _returnvalue_4)
                (Rendering|Material|SetMaterial _index_6 _output_get_6)
                (Rendering|Material|SetMaterial (Variables|Default|GetSkeletalMesh) _index_6 _output_get_6))
              (Timeline|Timeline PlayFromStart)
              (else
                (goto _label_5)))))
        (else
          ;;[1 1 1] Overwrite Material
          (if (== MaterialOverwrite 1)
            (goto _label_4)
            (elif (== MaterialOverwrite 2)
              (goto _label_5)
              (elif (== MaterialOverwrite 3)
                (goto _label_6)
                (else
                  (goto _label_5))))))))))

(fn ConstructionScript)