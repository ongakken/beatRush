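; Forcefield cube that spawns a separate impact actor when its collision registers a hit.
; On Hit, it adds a child actor component with configurable offset and scale, then messages that actor with the mesh-relative hit position, static mesh, hit component's material and an overwrite setting.
; A delay-based gate throttles spawning, ignoring further hits until the SpawnedActorReduction interval elapses.
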(event Collision|EventHit
  (params (MyComp :type Primitive%20Component%20Object%20Reference) (Other :type Actor%20Object%20Reference) (OtherComp :type Primitive%20Component%20Object%20Reference) (bSelfMoved :type Boolean) (HitLocation :type Vector) (HitNormal :type Vector :default "0, 0, 0") (NormalImpulse :type Vector :default "0, 0, 0") (Hit :type Hit%20Result%20Structure%20%28by%20ref%29))
  (bind _staticmesh (Variables|Default|GetStaticMesh))
  (if (not (Variables|Default|GetSpawnDelayActive))
    (Variables|Default|SetSpawnDelayActive true)
    (bind _returnvalue (AddComponent|AddChildActorComponent false (Math|Transform|MakeTransform (Variables|Default|GetLocationOffset) "0, 0, 0" (* "1.000000,1.000000,1.000000" (Variables|Default|GetScaleOffset)))))
    (Class|ShieldInterface|OnImpact(Message) (Variables|/Script/Engine.ChildActorComponent|GetChildActor _returnvalue) (- HitLocation (Transformation|GetWorldLocation _staticmesh)) _staticmesh (Rendering|Material|GetMaterial MyComp 0) (Variables|Default|GetMaterialOverwrite))
    (Utilities|FlowControl|Delay (Variables|Default|GetSpawnedActorReduction))
    (Variables|Default|SetSpawnDelayActive false)))

(fn ConstructionScript)