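; Obstacle actor that spins continuously and damages the player character on overlap.
; BeginPlay runs an endless short-Delay loop that sets its yaw from a steadily incremented rotation value instead of using Tick.
; On overlap with playerCharacter_BP, it applies damage scaled by the player's level, a random factor and InfProgressDividend, then destroys itself after a brief delay.
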(event EventBeginPlay
  (Transformation|SetActorRotation (Math|Rotator|MakeRotator 0.0 0.0 (Variables|Default|GetrotationDelta)) :!label _label)
  (Variables|Default|SetrotationDelta (+ (Variables|Default|GetrotationDelta) 0.1))
  (Utilities|FlowControl|Delay 0.01)
  (goto _label))

(event Collision|EventActorBeginOverlap
  (params (OtherActor :type Actor%20Object%20Reference))
  (bind _asplayer_character_bp (Utilities|Casting|CastToplayerCharacter_BP OtherActor))
  (Default|ApplyDamage _asplayer_character_bp (* (Variables|/Game/BP/playerCharacter_BP.playerCharacter_BP_C|GetlevelNum _asplayer_character_bp) 11.0 (Math|Random|RandomFloatinRange 0.2 1.3) (Variables|/Game/BP/playerCharacter_BP.playerCharacter_BP_C|Getinf_progressDividend _asplayer_character_bp)))
  (Utilities|FlowControl|Delay 0.1)
  (Actor|DestroyActor))

(fn ConstructionScript)