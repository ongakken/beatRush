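; BP_obstacleVar3 is an obstacle actor that spins its static mesh and damages the player on overlap.
; Each Tick adds a roll rotation equal to a Rotator counter, then increments it, so the spin keeps accelerating and depends on frame rate.
; Overlapping a playerCharacter_BP calls its ApplyDamage with a randomized amount scaled by that character's LevelNum and InfProgressDividend.
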(event Collision|EventActorBeginOverlap
  (params (OtherActor :type Actor%20Object%20Reference))
  (bind _asplayer_character_bp (Utilities|Casting|CastToplayerCharacter_BP OtherActor))
  (Default|ApplyDamage _asplayer_character_bp (* (Variables|/Game/BP/playerCharacter_BP.playerCharacter_BP_C|GetlevelNum _asplayer_character_bp) 14.0 (Math|Random|RandomFloatinRange 0.4 2.0) (Variables|/Game/BP/playerCharacter_BP.playerCharacter_BP_C|Getinf_progressDividend _asplayer_character_bp))))

(event EventTick
  (params (DeltaSeconds :type Float%20%28single-precision%29))
  (bind _rotator (Variables|Default|Getrotator))
  (Transformation|AddRelativeRotation (Variables|Debug|GetStaticMeshComponent) (Math|Rotator|MakeRotator _rotator 0.0 0.0) false false)
  (Math|Float|IncrementFloat _rotator))

(fn ConstructionScript)