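; BP_GameInfoInstance, part of the simple menu system, handles the settings save file stored in the GameSave slot.
; DoesSaveGameExist loads an existing BP_SettingsSave and returns it with true, or calls SaveAllSettings and returns false without an object.
; SaveAllSettings writes a newly created BP_SettingsSave to the slot without copying any values into it, so it stores only class defaults.
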(event Custom|SaveAllSettings
  (bind _returnvalue (SaveGame|CreateSaveGameObject "/Game/SimpleMenuSystem/Blueprints/BP_SettingsSave.BP_SettingsSave_C"))
  (bind _asbp_settings_save (Utilities|Casting|CastToBP_SettingsSave _returnvalue))
  (SaveGame|SaveGametoSlot _asbp_settings_save "GameSave"))

(fn DoesSaveGameExist?
  (bind _returnvalue (SaveGame|DoesSaveGameExist "GameSave"))
  (if _returnvalue
    (bind _returnvalue_2 (SaveGame|LoadGamefromSlot "GameSave"))
    (bind _asbp_settings_save (Utilities|Casting|CastToBP_SettingsSave _returnvalue_2))
    (return true _asbp_settings_save)
    (else
      (CallFunction|SaveAllSettings)
      (return false 0))))