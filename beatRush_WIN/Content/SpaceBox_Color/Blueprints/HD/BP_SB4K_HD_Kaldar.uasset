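; Kaldar HD skybox actor from the SpaceBox_Color set, forming a space backdrop that spins continuously during play.
; The construction script applies the configured scale and assigns a Kaldar material to each of the six face components.
; From BeginPlay, a short Delay loop sets pitch, yaw and roll to one growing angle, with a step that increases with the player character's LevelNum.
; Rotation never starts if the player cast fails.
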(event EventBeginPlay
  (bind _asplayer_character_bp (Utilities|Casting|CastToplayerCharacter_BP (Game|GetPlayerCharacter 0)))
  (Transformation|SetActorRotation (Math|Rotator|MakeRotator (Variables|Default|GetrotationDelta) (Variables|Default|GetrotationDelta) (Variables|Default|GetrotationDelta)) :!label _label)
  (Variables|Default|SetrotationDelta (+ (Variables|Default|GetrotationDelta) 0.05 (/ (Variables|/Game/BP/playerCharacter_BP.playerCharacter_BP_C|GetlevelNum _asplayer_character_bp) 1e+02)))
  (Utilities|FlowControl|Delay 0.01)
  (goto _label))

(fn ConstructionScript
  (Transformation|SetActorScale3D (Variables|Default|GetScale))
  (Rendering|Material|SetMaterial (Variables|Default|GetUp) 0 "/Game/SpaceBox_Color/Materials/HD/Kaldar/Mat_HD_Kaldar_Up.Mat_HD_Kaldar_Up")
  (Rendering|Material|SetMaterial (Variables|Default|GetRight) 0 "/Game/SpaceBox_Color/Materials/HD/Kaldar/Mat_HD_Kaldar_Right.Mat_HD_Kaldar_Right")
  (Rendering|Material|SetMaterial (Variables|Default|GetLeft) 0 "/Game/SpaceBox_Color/Materials/HD/Kaldar/Mat_HD_Kaldar_Left.Mat_HD_Kaldar_Left")
  (Rendering|Material|SetMaterial (Variables|Default|GetFront) 0 "/Game/SpaceBox_Color/Materials/HD/Kaldar/Mat_HD_Kaldar_Front.Mat_HD_Kaldar_Front")
  (Rendering|Material|SetMaterial (Variables|Default|GetDown) 0 "/Game/SpaceBox_Color/Materials/HD/Kaldar/Mat_HD_Kaldar_Down.Mat_HD_Kaldar_Down")
  (Rendering|Material|SetMaterial (Variables|Default|GetBack) 0 "/Game/SpaceBox_Color/Materials/HD/Kaldar/Mat_HD_Kaldar_Back.Mat_HD_Kaldar_Back"))