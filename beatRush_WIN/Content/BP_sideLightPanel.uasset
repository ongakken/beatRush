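; BP_sideLightPanel is a light panel actor whose emissive mesh glows in random colors.
; The construction script applies a dynamic instance of RoadCorner_emissive_Inst to the static mesh with a random color and set emissive power.
; From BeginPlay, an endless delay loop periodically creates a fresh material instance, rather than reusing the stored one, with a new, narrower-range random color and stronger glow.
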(event EventBeginPlay
  (Utilities|FlowControl|Delay 15.0 :!label _label)
  (bind _returnvalue (Rendering|Material|CreateDynamicMaterialInstance (Variables|Debug|GetStaticMeshComponent) 0 "/Game/Materials/roadCorner_emissive_Inst.roadCorner_emissive_Inst" "None" :!class /Script/Engine.PrimitiveComponent))
  (bind _output_get (Variables|Default|SetdynamicColorMat _returnvalue))
  (Rendering|Material|SetVectorParameterValue _output_get "Emissive Color" (Utilities|Struct|MakeLinearColor (Math|Random|RandomFloatinRange 0.1 0.9) (Math|Random|RandomFloatinRange 0.1 0.9) (Math|Random|RandomFloatinRange 0.1 0.9) 1.0) :!class /Script/Engine.MaterialInstanceDynamic)
  (Rendering|Material|SetScalarParameterValue _output_get "emissive power" 8.0 :!class /Script/Engine.MaterialInstanceDynamic)
  (goto _label))

(fn ConstructionScript
  (bind _returnvalue (Rendering|Material|CreateDynamicMaterialInstance (Variables|Debug|GetStaticMeshComponent) 0 "/Game/Materials/roadCorner_emissive_Inst.roadCorner_emissive_Inst" "None" :!class /Script/Engine.PrimitiveComponent))
  (bind _output_get (Variables|Default|SetdynamicColorMat _returnvalue))
  (Rendering|Material|SetVectorParameterValue _output_get "Emissive Color" (Utilities|Struct|MakeLinearColor (Math|Random|RandomFloatinRange 0.0 1.0) (Math|Random|RandomFloatinRange 0.0 1.0) (Math|Random|RandomFloatinRange 0.0 1.0) 1.0) :!class /Script/Engine.MaterialInstanceDynamic)
  (Rendering|Material|SetScalarParameterValue _output_get "emissive power" 6.0 :!class /Script/Engine.MaterialInstanceDynamic))