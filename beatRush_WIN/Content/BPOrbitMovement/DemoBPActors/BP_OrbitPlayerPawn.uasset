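; Demo player pawn for the BPOrbitMovement component that turns to face its velocity relative to the orbited mass and tests orbit prediction.
; The PredictOrbit input stores and draws a line to the component's predicted future position, then starts a timer for that prediction interval.
; Tick shows the remaining countdown at that point, and on expiry ShowFuturePositionError prints the prediction error alongside the straight-line distance travelled.
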(event EventBeginPlay
  (Development|PrintText "Press 'P' to predict orbit " true false "(R=0.000000,G=0.660000,B=1.000000,A=1.000000)" 5.0))

(event EventActorBeginOverlap
  (params (OtherActor :type Actor%20Object%20Reference)))

(event EventTick
  (params (DeltaSeconds :type Float%20%28single-precision%29))
  ;[1 1 1] Make the PlayerPawn face forward, forward based on the velocity relative to the mass the player is orbiting
  (bind _relativevelocity (Default|GetRelativetoMassVelocity (Variables|/Game/BPOrbitMovement/BP_OrbitMovementComponent.BP_OrbitMovementComponent_C|GetOrbit (Variables|OrbitPlugin|GetBP_OrbitMovement))))
  (Transformation|SetActorRotation (Math|Rotator|FindLookatRotation (Transformation|GetActorLocation) (+ _relativevelocity (Transformation|GetActorLocation))))
  ;[1 1 1] If there is a FuturePosition timer, show how much time is remaining
  (if (Class|KismetSystemLibrary|TimerExistsHandle (Variables|OrbitPlugin|GetTimerStore))
    (Rendering|Debug|DrawDebugString (Variables|OrbitPlugin|GetFuturePositionStore) (Utilities|String|Append "Orbit prediction time remaining: " (Utilities|String|ToString(Float) (Utilities|Time|GetTimerRemainingTimebyHandle (Variables|OrbitPlugin|GetTimerStore)))) 0 "(R=1.000000,G=1.000000,B=1.000000,A=1.000000)" 0.01)))

(event Input|ActionEvents|InputActionPredictOrbit
  (params (Key :type Key%20Structure :default "None"))
  (:Pressed
    ;[1 1 1] Calculate the future position
    (bind _new_position (Default|CalculateFuturePosition (Variables|/Game/BPOrbitMovement/BP_OrbitMovementComponent.BP_OrbitMovementComponent_C|GetOrbit (Variables|OrbitPlugin|GetBP_OrbitMovement)) (Variables|OrbitPlugin|GetFutureOrbitPredictionValue)))
    ;[1 1 1] Save FuturePosition value so we can calculate how accurate it was
    (bind _output_get (Variables|OrbitPlugin|SetFuturePositionStore _new_position))
    ;[1 1 1] Draw a line to the future position
    (Rendering|Debug|DrawDebugLine (Transformation|GetActorLocation) _output_get "(R=1.000000,G=1.000000,B=1.000000,A=1.000000)" (Variables|OrbitPlugin|GetFutureOrbitPredictionValue) 5.0)
    ;[1 1 1] Set a timer to when we should be arriving at the predicted location
    (bind _returnvalue (Utilities|Time|SetTimerbyFunctionName 0 "ShowFuturePositionError" (Variables|OrbitPlugin|GetFutureOrbitPredictionValue)))
    (Variables|OrbitPlugin|SetTimerStore _returnvalue)
    ;[1 1 1] Lets us figure out how far we travelled for this prediction
    (Variables|OrbitPlugin|SetCurrentLocationStore (Transformation|GetActorLocation))))

(fn ConstructionScript)

(fn ShowFuturePositionError
  (Development|PrintText (Utilities|Text|ToText(String) (Utilities|String|Append "Orbit prediction of " (Utilities|String|ToString(Float) (Variables|OrbitPlugin|GetFutureOrbitPredictionValue)) " seconds  was accurate to " (Utilities|String|ToString(Float) (Math|Vector|VectorLength (- (Transformation|GetActorLocation) (Variables|OrbitPlugin|GetFuturePositionStore)))) " unreal units." "Travel Distance: " (Utilities|String|ToString(Float) (Math|Vector|VectorLength (- (Variables|OrbitPlugin|GetCurrentLocationStore) (Transformation|GetActorLocation)))))) true true "(R=1.000000,G=1.000000,B=1.000000,A=1.000000)" 3.0))