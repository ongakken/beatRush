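; Example orbiting actor for the BPOrbitMovement demo, carrying a BPOrbitMovement component.
; When ShowVelocityDebugLines is set, Tick draws two debug lines from the actor's location.
; The green line shows the component's relative orbit velocity and the red line shows its world velocity.
; The graph holds no movement logic of its own, only this visualization.
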(event EventBeginPlay)

(event EventActorBeginOverlap
  (params (OtherActor :type Actor%20Object%20Reference)))

(event EventTick
  (params (DeltaSeconds :type Float%20%28single-precision%29))
  (bind _returnvalue (Transformation|GetActorLocation))
  (bind _returnvalue_2 (Transformation|GetActorLocation))
  (if (Variables|OrbitPlugin|GetShowVelocityDebugLines)
    (Rendering|Debug|DrawDebugLine _returnvalue (+ _returnvalue (* (Variables|/Game/BPOrbitMovement/Lib/BP_Orbit.BP_Orbit_C|GetOrbitVelocity (Variables|/Game/BPOrbitMovement/BP_OrbitMovementComponent.BP_OrbitMovementComponent_C|GetOrbit (Variables|Default|GetBP_OrbitMovement))) 1.0)) "(R=0.078338,G=0.915000,B=0.343154,A=1.000000)" 0.1 1e+01)
    (Rendering|Debug|DrawDebugLine _returnvalue_2 (+ _returnvalue_2 (* (Variables|/Game/BPOrbitMovement/BP_OrbitMovementComponent.BP_OrbitMovementComponent_C|GetVelocity (Variables|Default|GetBP_OrbitMovement)) 1.0)) "(R=0.975000,G=0.057671,B=0.094924,A=1.000000)" 0.1 1e+01)))

(fn ConstructionScript)